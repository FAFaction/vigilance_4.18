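; Game instance that keeps the last checkpoint and player location across level loads and restarts play from it.
; Restarting reopens the test map, removes the main menu, shows a timed loading screen widget and restores game-only input.
; It then teleports the player character to the saved location and possesses it, using fixed delays to sequence the steps.
; An unconnected branch holds graphics settings loading and hardware benchmark logic.
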(event Custom|Restart%20From%20Last%20Checkpoint
  (bind _returnvalue (Game|GetPlayerController 0))
  ;[1 1 1] Restart From the last checkpoint
  (Game|OpenLevel(byName) "GamePlayTestMap")
  (Utilities|FlowControl|Delay 0.1)
  (bind _foundwidgets (Widget|GetAllWidgetsOfClass "/Game/UI/MainMenu/MainMenuUI.MainMenuUI_C" false))
  (Widget|RemovefromParent (Utilities|Array|Get(acopy) _foundwidgets))
  (CallFunction|ShowLoadingScreen 2.0)
  (Input|SetInputModeGameOnly _returnvalue)
  (Variables|/Script/Engine.PlayerController|SetbShowMouseCursor _returnvalue false)
  (bind _outactors (Actor|GetAllActorsOfClass "/Game/Blueprints/PlayerBlueprint/Player_CharacterBP.Player_CharacterBP_C"))
  (Transformation|SetActorLocation (Utilities|Array|Get(acopy) _outactors) (Variables|Default|GetPlayer%20Location%20A) false true)
  (Utilities|FlowControl|Delay 1.8)
  (Pawn|Possess (Game|GetPlayerController 0) (Utilities|Array|Get(acopy) _outactors)))

(event Custom|Update%20Checkpoint
  (params (CheckPoint :type Checkpoint%20BP%20Object%20Reference) (Player%20Location%20A :type Vector))
  (Variables|Default|SetCheckPoint CheckPoint)
  (Variables|Default|SetPlayer%20Location%20A Player%20Location%20A))

(event EventInit)

(fn ShowLoadingScreen
  (params (Duration :type Float%20%28single-precision%29))
  (bind _returnvalue (UserInterface|CreateWidget "/Game/UI/MainMenu/LoadingScreen.LoadingScreen_C" 0 Duration))
  (UserInterface|Viewport|AddtoPlayerScreen _returnvalue 5))