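; Drivable hover vehicle pawn that the player character can enter and exit, with animated doors, impact sparks and switchable first/third-person cameras with side views.
; Entering and exiting use camera fades, seat attachment and possession swaps; exiting also traces down to set the vehicle on the ground.
; Driving applies force and torque to the Box, while pitch rotates the actor directly; older kinematic movement and hover code is disconnected.
; It also spawns a missing player and triggers an incoming call after possession.
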(event OnComponentHit(Box)
  (params (HitComponent :type Primitive%20Component%20Object%20Reference) (OtherActor :type Actor%20Object%20Reference) (OtherComp :type Primitive%20Component%20Object%20Reference) (NormalImpulse :type Vector :default "0, 0, 0") (Hit :type Hit%20Result%20Structure%20%28by%20ref%29))
  (bind (_bblockinghit _binitialoverlap _time _distance _location _impactpoint _normal _impactnormal) (Collision|BreakHitResult Hit))
  (if (Math|Boolean|ORBoolean (> (Math|Float|Absolute(Float) (Input|AxisValues|GetMoveForward)) 0.0) (> (Math|Float|Absolute(Float) (Input|AxisValues|GetTurn)) 0.0) (> (Math|Float|Absolute(Float) (Input|AxisValues|GetLookUp)) 0.0))
    (Effects|SpawnEmitteratLocation "/Game/GameContent/SciFiWeapLight/FX/Particles/P_Impact_Metal_Small_Light.P_Impact_Metal_Small_Light" _impactpoint (Math|Rotator|MakeRotfromX _impactnormal))))

(event Custom|Open/CloseDoorR
  (params (Open :type Boolean))
  ;[1 1 1] Opening Doors by roatting arrows in the yawlocation
  (if Open
    (bind _door_yaw (Timeline|Open%20DoorR Play)
      (:Update
        (Transformation|SetRelativeRotation (Variables|Default|GetArrow%20R) (Math|Rotator|MakeRotator 0.0 0.0 _door_yaw) false false)))
    (else
      (Timeline|Open%20DoorR Reverse))))

(event Custom|Enter%20Car
  (params (Player :type Player%20Character%20BP%20Object%20Reference))
  ;[1 1 1] Comment
  (Variables|Default|SetPlayer%20Ref Player)
  (CameraFades|StartCameraFade :self (Game|GetPlayerCameraManager 0) :ToAlpha 1.0 :Duration 1.0)
  (Utilities|FlowControl|Delay 1.0)
  (Collision|SetCollisionEnabled (Variables|/Script/Engine.Character|GetCapsuleComponent (Variables|Default|GetPlayer%20Ref)) "NoCollision")
  (Transformation|AttachComponentToComponent (Variables|Default|GetPlayer%20Ref) (Variables|Default|GetSeat) "None" "SnapToTarget" "SnapToTarget" "SnapToTarget" true)
  (Components|Animation|PlayAnimation (Variables|/Script/Engine.Character|GetMesh (Variables|Default|GetPlayer%20Ref)) "/Game/GameContent/Animations/MovementAnimSetPro/SitChairLoop.SitChairLoop" true)
  (CameraFades|StartCameraFade :self (Game|GetPlayerCameraManager 0) :FromAlpha 1.0 :Duration 1.0)
  (Default|UnpossesPlayer (Variables|Default|GetPlayer%20Ref))
  (Pawn|Possess (Game|GetPlayerController 0) self)
  (Variables|Default|SetIs%20Being%20Drive%20? true)
  (Variables|Default|SetIn%20Car true))

(event Custom|Open/CloseDoorL
  (params (Open :type Boolean))
  ;[1 1 1] Opening Doors by roatting arrows in the yawlocation
  (if Open
    (bind _door_yaw (Timeline|Open%20DoorL Play)
      (:Update
        (Transformation|SetRelativeRotation (Variables|Default|GetArrow%20L) (Math|Rotator|MakeRotator 0.0 0.0 _door_yaw) false false)))
    (else
      (Timeline|Open%20DoorL Reverse))))

(event Custom|Exit%20Car
  (bind _returnvalue (Game|GetPlayerController 0))
  (bind _returnvalue_2 (Transformation|GetActorLocation))
  ;[1 1 1] Comment
  (if (Variables|Default|GetIn%20Car)
    (Variables|Default|SetIs%20Being%20Drive%20? false)
    (CameraFades|StartCameraFade :self (Game|GetPlayerCameraManager 0) :ToAlpha 1.0 :Duration 1.0)
    (Utilities|FlowControl|Delay 1.0)
    (bind _outhit (Collision|LineTraceByChannel _returnvalue_2 (- _returnvalue_2 "0, 0,200.000000") "TraceTypeQuery1" false 0 "None"))
    (Transformation|SetActorLocation (.ImpactPoint (Collision|BreakHitResult _outhit)) true false)
    (CallFunction|WhenExitCar)
    (Transformation|DetachFromActor (Variables|Default|GetPlayer%20Ref) "KeepRelative" "KeepRelative" "KeepRelative")
    (Transformation|SetActorLocation (Variables|Default|GetPlayer%20Ref) (Transformation|GetWorldLocation (Variables|Default|GetExit%20Position)) false false)
    (Collision|SetCollisionEnabled (Variables|/Script/Engine.Character|GetCapsuleComponent (Variables|Default|GetPlayer%20Ref)) "QueryAndPhysics")
    (Pawn|UnPossess _returnvalue)
    (Pawn|Possess _returnvalue (Variables|Default|GetPlayer%20Ref))
    (Components|SkeletalMesh|SetAnimInstanceClass (Variables|/Script/Engine.Character|GetMesh (Variables|Default|GetPlayer%20Ref)) "/Game/Blueprints/PlayerBlueprint/Player_AnimBP.Player_AnimBP_C")
    (CameraFades|StartCameraFade :self (Game|GetPlayerCameraManager 0) :FromAlpha 1.0 :Duration 1.0)
    (Variables|Default|SetIn%20Car false)))

(event Custom|When%20Exit%20Car
  (bind _returnvalue (Transformation|GetActorLocation))
  (bind _outhit (Collision|SphereTraceByChannel _returnvalue (- _returnvalue "0, 0,500.000000") 2e+01 "TraceTypeQuery1" false 0 "None"))
  (Transformation|SetActorLocation (+ (.ImpactPoint (Collision|BreakHitResult _outhit)) "0, 0,10.000000") true false))

(event EventPossessed
  (params (NewController :type Controller%20Object%20Reference))
  (if (Pawn|IsPlayerControlled)
    (Utilities|FlowControl|Delay 2.0)
    (bind _outactors (Actor|GetAllActorsOfClass "/Game/Blueprints/CustomBlueprints/Caller/Call_In_The_player_Apartment.Call_In_The_player_Apartment_C"))
    (Default|GettingACall (Utilities|Array|Get(acopy) _outactors))))

(event EventTick
  (params (DeltaSeconds :type Float%20%28single-precision%29))
  (CallFunction|MovementGraphEventTick DeltaSeconds))

(event EventBeginPlay
  (bind _box (Variables|Default|GetBox))
  (bind _returnvalue (Transformation|GetWorldLocation _box))
  (Utilities|FlowControl|Delay 0.2)
  (bind _outactors (Actor|GetAllActorsOfClass "/Game/Blueprints/PlayerBlueprint/Player_CharacterBP.Player_CharacterBP_C"))
  (Utilities|IsValid (Utilities|Array|Get(acopy) _outactors)
    (:Is%20Not%20Valid
      (Game|SpawnActorfromClass "/Game/Blueprints/PlayerBlueprint/Player_CharacterBP.Player_CharacterBP_C" (Math|Transform|MakeTransform (Math|Vector|MakeVector (.x _returnvalue) (.y _returnvalue) (+ (.z _returnvalue) 3e+02)) "0, 0, 0" "1,1,1") "AlwaysSpawn" 0 0))))

(event Input|AxisEvents|InputAxisTurn
  (params (AxisValue :type Float%20%28single-precision%29))
  (Pawn|Input|AddControllerYawInput AxisValue))

(event Input|KeyboardEvents|G
  (params (Key :type Key%20Structure))
  ;[1 1 1] Start and Stop Engine
)

(event Custom|MovementGraphEvent%20Tick
  (params (Delta :type Float%20%28single-precision%29)))

(event Input|AxisEvents|InputAxisMoveRight
  (params (AxisValue :type Float%20%28single-precision%29))
  ;[1 1 1] Roll Car
)

(event Input|AxisEvents|InputAxisTurn
  (params (AxisValue :type Float%20%28single-precision%29))
  ;[1 1 1] Turning
)

(event Input|AxisEvents|InputAxisLookUp
  (params (AxisValue :type Float%20%28single-precision%29))
  (bind _returnvalue (Transformation|GetActorRotation))
  ;[1 1 1] Go Up down
  (bind _output_get (Variables|Default|SetUp%20Axis (Math|Interpolation|FInterpTo (Variables|Default|GetUp%20Axis) (* AxisValue -1.0) (Utilities|Time|GetWorldDeltaSeconds) 5.0)))
  (Transformation|AddActorLocalRotation (Math|Rotator|MakeRotator 0.0 _output_get 0.0) false false)
  (Transformation|SetActorRotation (Math|Rotator|MakeRotator 0.0 (.pitch _returnvalue) (.yaw _returnvalue))))

(event Input|AxisEvents|InputAxisMoveForward
  (params (AxisValue :type Float%20%28single-precision%29))
  ;[1 1 1] Move Forward
)

(event Input|KeyboardEvents|Z
  (params (Key :type Key%20Structure))
  ;[1 1 1] Set Fpp
  (:Pressed
    (Utilities|FlowControl|FlipFlop
      (:A
        (CallFunction|SetFPP true))
      (:B
        (CallFunction|SetFPP false)))))

(event Input|KeyboardEvents|E
  (params (Key :type Key%20Structure))
  (bind _springarm (Variables|Default|GetSpringArm))
  (bind _springarmfppcam (Variables|Default|GetSpringArmFPPCam))
  (:Pressed
    (Transformation|SetRelativeRotation _springarm "0,180.000000, 0" false false)
    (Transformation|SetRelativeRotation _springarmfppcam "0,90.000000, 0" false false))
  (:Released
    (Transformation|SetRelativeRotation _springarm "0,90.000000, 0" false false)
    (Transformation|SetRelativeRotation _springarmfppcam "0, 0, 0" false false)))

(event Input|KeyboardEvents|Q
  (params (Key :type Key%20Structure))
  (bind _springarm (Variables|Default|GetSpringArm))
  (bind _springarmfppcam (Variables|Default|GetSpringArmFPPCam))
  (:Pressed
    (Transformation|SetRelativeRotation _springarm "0, 0, 0" false false)
    (Transformation|SetRelativeRotation _springarmfppcam "0,-90.000000, 0" false false))
  (:Released
    (Transformation|SetRelativeRotation _springarm "0,90.000000, 0" false false)
    (Transformation|SetRelativeRotation _springarmfppcam "0, 0, 0" false false)))

(event Input|AxisEvents|InputAxisTurn
  (params (AxisValue :type Float%20%28single-precision%29))
  (Class|PrimitiveComponent|AddTorqueinDegrees (Variables|Default|GetBox) (Math|Vector|MakeVector 0.0 0.0 (* AxisValue 6e+02)) "None" true))

(event Input|AxisEvents|InputAxisLookUp
  (params (AxisValue :type Float%20%28single-precision%29)))

(event Input|AxisEvents|InputAxisLookUp
  (params (AxisValue :type Float%20%28single-precision%29))
  (bind _returnvalue (Transformation|GetActorRotation))
  ;[1 1 1] Go Up down
  (bind _output_get (Variables|Default|SetUp%20Axis (Math|Interpolation|FInterpTo (Variables|Default|GetUp%20Axis) (* AxisValue -1.0) (Utilities|Time|GetWorldDeltaSeconds) 5.0)))
  (Transformation|AddActorLocalRotation (Math|Rotator|MakeRotator 0.0 _output_get 0.0) false false)
  (Transformation|SetActorRotation (Math|Rotator|MakeRotator 0.0 (.pitch _returnvalue) (.yaw _returnvalue))))

(event Input|AxisEvents|InputAxisMoveForward
  (params (AxisValue :type Float%20%28single-precision%29))
  (Physics|AddForce (Variables|Default|GetBox) (* (* (Transformation|GetActorForwardVector) 6e+03) AxisValue) "None" true))

(fn ConstructionScript)

(fn SetFPP
  (params (FPP :type Boolean))
  (bind _fpp_cam (Variables|Default|GetFPP%20Cam))
  (bind _camera (Variables|Default|GetCamera))
  (if FPP
    (Components|Activation|SetActive _fpp_cam true false)
    (Components|Activation|SetActive _camera false false)
    (else
      (Components|Activation|SetActive _fpp_cam false false)
      (Components|Activation|SetActive _camera true false))))