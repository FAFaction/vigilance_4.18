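; BulletBase_BP is a base projectile actor for guns that damages characters on impact.
; On spawn it sets a limited lifespan and makes its mesh and capsule ignore the owning actor when moving.
; A mesh hit applies the Damage value to a Character, falling back to a random pick from preset amounts if unset.
; Any mesh hit spawns a small metal impact effect and destroys the bullet.
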(event OnComponentBeginOverlap(Capsule)
  (params (OverlappedComponent :type Primitive%20Component%20Object%20Reference) (OtherActor :type Actor%20Object%20Reference) (OtherComp :type Primitive%20Component%20Object%20Reference) (OtherBodyIndex :type Integer) (bFromSweep :type Boolean) (SweepResult :type Hit%20Result%20Structure%20%28by%20ref%29)))

(event OnComponentHit(StaticMesh)
  (params (HitComponent :type Primitive%20Component%20Object%20Reference) (OtherActor :type Actor%20Object%20Reference) (OtherComp :type Primitive%20Component%20Object%20Reference) (NormalImpulse :type Vector :default "0, 0, 0") (Hit :type Hit%20Result%20Structure%20%28by%20ref%29))
  (bind _damage (Variables|Default|GetDamage))
  (bind _ascharacter (Utilities|Casting|CastToCharacter OtherActor)
    (:then
      (Game|Damage|ApplyDamage _ascharacter (select (> _damage 0.0) _damage (Utilities|Select :Index (Math|Random|RandomIntegerinRange 0 3) :Option%200 4.0 :Option%201 6.0 :Option%202 1e+01 :Option%203 12.0)) 0 self))
    (:CastFailed
      _))
  (Effects|SpawnEmitteratLocation "/Game/GameContent/SciFiWeapLight/FX/Particles/P_Impact_Metal_Large_Light.P_Impact_Metal_Large_Light" (Transformation|GetActorLocation) "0, 0, 0" "0.200000,0.200000,0.200000")
  (Actor|DestroyActor))

(event EventBeginPlay
  (Actor|SetLifeSpan 1e+01)
  (Collision|IgnoreActorwhenMoving (Variables|Default|GetStaticMesh) (Variables|Default|GetOwning%20Actor) true))

(event Collision|EventActorBeginOverlap
  (params (OtherActor :type Actor%20Object%20Reference)))

(event EventTick
  (params (DeltaSeconds :type Float%20%28single-precision%29)))

(event Collision|EventHit
  (params (MyComp :type Primitive%20Component%20Object%20Reference) (Other :type Actor%20Object%20Reference) (OtherComp :type Primitive%20Component%20Object%20Reference) (bSelfMoved :type Boolean) (HitLocation :type Vector :default "0, 0, 0") (HitNormal :type Vector :default "0, 0, 0") (NormalImpulse :type Vector :default "0, 0, 0") (Hit :type Hit%20Result%20Structure%20%28by%20ref%29)))

(fn ConstructionScript)