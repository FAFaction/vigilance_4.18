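; Sci-fi pistol weapon Blueprint that fires projectiles using a self-regenerating charge, topped up on a delayed Tick up to a maximum.
; Fire spends charge, plays a standing or crouched montage on the player, then traces from the camera to aim a spawned BulletBase_BP from the muzzle arrow, with effects.
; CoverFire reuses that shot without the montage.
; Charged-shot events are empty stubs, and their damage ramp logic is unwired.
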(event Custom|Release%20Charge)

(event Custom|Cover%20Fire
  (params (Player%20ref :type Player%20Character%20BP%20Object%20Reference))
  (bind _returnvalue (Game|Player|GetPlayerPawn 0))
  (bind _arrow (Variables|Default|GetArrow))
  (bind _arrow_2 (Variables|Default|GetArrow))
  (bind _returnvalue_2 (Transformation|GetSocketLocation _arrow_2 "None"))
  (bind _returnvalue_3 (Transformation|GetWorldLocation _arrow))
  (Variables|Default|SetPlayer%20ref Player%20ref)
  (if (> (Variables|Default|GetCharge) 5.0)
    (Variables|Default|SetCharge (- (Variables|Default|GetCharge) 5.0))
    (bind (_outhit _returnvalue_4) (Collision|LineTraceByChannel (+ (Transformation|GetWorldLocation (Default|GetPlayerCamera (Variables|Default|GetPlayer%20ref))) (* (Math|Vector|GetForwardVector (Default|GetPlayerCamera (Variables|Default|GetPlayer%20ref))) 2e+02)) (+ (Transformation|GetWorldLocation (Default|GetPlayerCamera (Variables|Default|GetPlayer%20ref))) (* (Math|Vector|GetForwardVector (Default|GetPlayerCamera (Variables|Default|GetPlayer%20ref))) 9999.0)) "TraceTypeQuery2" false (Utilities|Array|MakeArray (Variables|Default|GetPlayer%20ref)) "None"))
    (Game|SpawnActorfromClass "/Game/Blueprints/GunBlueprint/BulletBase_BP.BulletBase_BP_C" (Math|Transform|MakeTransform _returnvalue_3 (Math|Rotator|FindLookatRotation _returnvalue_3 (Math|Vector|SelectVector (.ImpactPoint (Collision|BreakHitResult _outhit)) (.TraceEnd (Collision|BreakHitResult _outhit)) _returnvalue_4)) "0.400000,0.400000,0.400000") "AlwaysSpawn" 0 (Variables|Default|GetDamage) _returnvalue _returnvalue)
    (Effects|SpawnEmitteratLocation "/Game/GameContent/SciFiWeapLight/FX/Particles/P_Pistol_MuzzleFlash_Light.P_Pistol_MuzzleFlash_Light" _returnvalue_2)
    (Audio|PlaySoundatLocation "/Game/GameContent/SciFiWeapLight/Sound/Pistol/Pistol_Fire_Cue.Pistol_Fire_Cue" _returnvalue_2)
    (Camera|PlayWorldCameraShake "/Game/Blueprints/GunBlueprint/CamShack_Gun.CamShack_Gun_C" (Transformation|GetActorLocation) 0.0 399.0 1.0 true)
    (Components|Animation|PlayAnimation (Variables|Default|GetSkeletalMesh) "/Game/GameContent/SciFiWeapLight/Weapons/Anims/Fire_Pistol_W.Fire_Pistol_W" false)))

(event Custom|FireCharge)

(event Custom|Fire
  (params (Player%20ref :type Player%20Character%20BP%20Object%20Reference))
  (bind _returnvalue (Game|Player|GetPlayerPawn 0))
  (bind _arrow (Variables|Default|GetArrow))
  (bind _arrow_2 (Variables|Default|GetArrow))
  (bind _returnvalue_2 (Transformation|GetSocketLocation _arrow_2 "None"))
  (bind _returnvalue_3 (Transformation|GetWorldLocation _arrow))
  (Variables|Default|SetPlayer%20ref Player%20ref)
  (if (> (Variables|Default|GetCharge) 5.0)
    (Utilities|FlowControl|Sequence
      (:then_0
        (switch Utilities|FlowControl|Switch|SwitchonPlayerMovementState (Variables|/Game/Blueprints/PlayerBlueprint/Player_CharacterBP.Player_CharacterBP_C|GetMovement%20State (Variables|Default|GetPlayer%20ref))
          (:NewEnumerator0
            (Animation|PlayAnimMontage (Variables|Default|GetPlayer%20ref) "/Game/GameContent/Animations/NewFolder/PistolShoot_Montage.PistolShoot_Montage" 1.0 "None"))
          (:NewEnumerator1
            (Animation|PlayAnimMontage (Variables|Default|GetPlayer%20ref) "/Game/GameContent/Animations/NewFolder/PistolShootCrouched_Montage.PistolShootCrouched_Montage" 0.5 "None"))))
      (:then_1
        (Variables|Default|SetCharge (- (Variables|Default|GetCharge) 5.0))
        (bind (_outhit _returnvalue_4) (Collision|LineTraceByChannel (+ (Transformation|GetWorldLocation (Default|GetPlayerCamera (Variables|Default|GetPlayer%20ref))) (* (Math|Vector|GetForwardVector (Default|GetPlayerCamera (Variables|Default|GetPlayer%20ref))) 2e+02)) (+ (Transformation|GetWorldLocation (Default|GetPlayerCamera (Variables|Default|GetPlayer%20ref))) (* (Math|Vector|GetForwardVector (Default|GetPlayerCamera (Variables|Default|GetPlayer%20ref))) 9999.0)) "TraceTypeQuery2" false (Utilities|Array|MakeArray (Variables|Default|GetPlayer%20ref)) "None"))
        (Game|SpawnActorfromClass "/Game/Blueprints/GunBlueprint/BulletBase_BP.BulletBase_BP_C" (Math|Transform|MakeTransform _returnvalue_3 (Math|Rotator|FindLookatRotation _returnvalue_3 (Math|Vector|SelectVector (.ImpactPoint (Collision|BreakHitResult _outhit)) (.TraceEnd (Collision|BreakHitResult _outhit)) _returnvalue_4)) "0.400000,0.400000,0.400000") "AlwaysSpawn" 0 (Variables|Default|GetDamage) _returnvalue _returnvalue)
        (Effects|SpawnEmitteratLocation "/Game/GameContent/SciFiWeapLight/FX/Particles/P_Pistol_MuzzleFlash_Light.P_Pistol_MuzzleFlash_Light" _returnvalue_2)
        (Audio|PlaySoundatLocation "/Game/GameContent/SciFiWeapLight/Sound/Pistol/Pistol_Fire_Cue.Pistol_Fire_Cue" _returnvalue_2)
        (Camera|PlayWorldCameraShake "/Game/Blueprints/GunBlueprint/CamShack_Gun.CamShack_Gun_C" (Transformation|GetActorLocation) 0.0 399.0 1.0 true)
        (Components|Animation|PlayAnimation (Variables|Default|GetSkeletalMesh) "/Game/GameContent/SciFiWeapLight/Weapons/Anims/Fire_Pistol_W.Fire_Pistol_W" false)))))

(event EventBeginPlay
  (bind _outactors (Actor|GetAllActorsOfClass "/Game/Blueprints/PlayerBlueprint/Player_CharacterBP.Player_CharacterBP_C"))
  (Variables|Default|SetPlayer%20ref (Utilities|Array|Get(acopy) _outactors)))

(event Collision|EventActorBeginOverlap
  (params (OtherActor :type Actor%20Object%20Reference)))

(event EventTick
  (params (DeltaSeconds :type Float%20%28single-precision%29))
  (Utilities|FlowControl|Delay 0.3)
  (Variables|Default|SetCharge (Math|Float|Clamp(Float) (+ (Variables|Default|GetCharge) 1.0) 0.0 (Variables|Default|GetMax%20Charge))))

(fn ConstructionScript)