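; Hackable rifle-wielding AI character that shoots at the player, or is driven by the player while possessed.
; Unpossessed by the player, Tick runs a range, view-cone and line-trace sight check, then turns and fires with random spread.
; Possessed, it takes movement, weapon-toggle and automatic-fire input, sharing the bullet-spawning Shoot function.
; Child-actor HackedActor receives control-timeout settings, and death makes player controller repossess the player character.
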(event Custom|Loos%20Control
  (bind _outactors (Actor|GetAllActorsOfClass "/Game/Blueprints/PlayerBlueprint/Player_CharacterBP.Player_CharacterBP_C"))
  (Pawn|Possess (Game|GetPlayerController 0) (Utilities|Array|Get(acopy) _outactors)))

(event EventBeginPlay
  (bind _ashacked_actor_bp (Utilities|Casting|CastToHackedActor_BP (Variables|/Script/Engine.ChildActorComponent|GetChildActor (Variables|Default|GetHacked))))
  (Variables|/Game/Blueprints/CustomBlueprints/HackingSystem/HackedActor_BP.HackedActor_BP_C|SetShould%20loos%20control%20on%20time%20out _ashacked_actor_bp (Variables|Default|GetShould%20Loos%20Control%20on%20time%20out))
  (Variables|/Game/Blueprints/CustomBlueprints/HackingSystem/HackedActor_BP.HackedActor_BP_C|SetControl%20time _ashacked_actor_bp (Variables|Default|GetControl%20Time))
  (EventDispatchers|BindEventtoOnDeath (Variables|Default|GetHealthAndDamageComponent) (delegate Custom|Loos%20Control)))

(event Collision|EventActorBeginOverlap
  (params (OtherActor :type Actor%20Object%20Reference)))

(event EventTick
  (params (DeltaSeconds :type Float%20%28single-precision%29))
  (CallFunction|AITick))

(event EventUnpossessed
  (params (OldController :type Controller%20Object%20Reference))
  (bind _asobject_scanner (Utilities|Casting|CastToObjectScanner (Variables|/Script/Engine.ChildActorComponent|GetChildActor (Variables|Default|GetScanner))))
  (Default|ScanStop _asobject_scanner)
  (bind _ashacked_actor_bp (Utilities|Casting|CastToHackedActor_BP (Variables|/Script/Engine.ChildActorComponent|GetChildActor (Variables|Default|GetHacked))))
  (Rendering|SetVisibility (Variables|/Game/Blueprints/CustomBlueprints/HackingSystem/HackedActor_BP.HackedActor_BP_C|GetWidget _ashacked_actor_bp) false false))

(event Custom|AI%20Tick
  (if (> (Variables|/Game/Blueprints/HealthAndDamageComponent.HealthAndDamageComponent_C|GetHealth (Variables|Default|GetHealthAndDamageComponent)) 0.0)
    (if (not (Pawn|IsPlayerControlled))
      (CallFunction|CanSeePlayer)
      (CallFunction|ShootatPlayer))))

(event Custom|Shoot%20at%20player
  (if (Variables|Default|GetPlayer%20in%20sight)
    (Variables|Default|SetShooting true)
    (Transformation|SetActorRotation (Math|Rotator|FindLookatRotation (Transformation|GetActorLocation) (Transformation|GetActorLocation (Game|Player|GetPlayerPawn 0))))
    (Utilities|FlowControl|Delay 1.0)
    (CallFunction|Shoot (Variables|Default|GetCamera))
    (else
      (Variables|Default|SetShooting false))))

(event Custom|Can%20See%20Player
  ;[1 1 1] Can See Player
  (if (< (Transformation|GetDistanceTo (Game|Player|GetPlayerPawn 0)) 1e+03)
    (if (< (Class|KismetMathLibrary|DegAcos (Math|Vector|DotProduct (Math|Vector|Normalize (- (Transformation|GetActorLocation (Game|Player|GetPlayerPawn 0)) (Transformation|GetActorLocation))) (Transformation|GetActorForwardVector))) 35.0)
      (bind (_outhit _returnvalue) (Collision|LineTraceByChannel (Transformation|GetActorLocation) (Transformation|GetActorLocation (Game|GetPlayerCharacter 0)) "TraceTypeQuery2" false 0 "ForOneFrame"))
      (if _returnvalue
        (if (== (.HitActor (Collision|BreakHitResult _outhit)) (Game|Player|GetPlayerPawn 0))
          (Variables|Default|SetPlayer%20in%20sight true)
          (Utilities|FlowControl|Sequence
            (:then_0
              (Utilities|FlowControl|DoOnce false :!label _label
                (:Completed
                  (CallFunction|EquipWeapon true))))
            (:then_1
              (goto _label_2 Reset)))
          (else
            (Variables|Default|SetPlayer%20in%20sight false)
            (Utilities|FlowControl|Sequence
              (:then_0
                (Utilities|FlowControl|DoOnce false :!label _label_2
                  (:Completed
                    (CallFunction|EquipWeapon false))))
              (:then_1
                (goto _label Reset)))))
        (else
          (Variables|Default|SetPlayer%20in%20sight false))))))

(event Input|AxisEvents|InputAxisMoveForward
  (params (AxisValue :type Float%20%28single-precision%29))
  ;[1 1 1] Basic Input
  (Pawn|Input|AddMovementInput (Math|Vector|GetForwardVector (Math|Rotator|MakeRotator 0.0 0.0 (.yaw (Pawn|GetControlRotation :!class /Script/Engine.Pawn)))) AxisValue false))

(event Input|AxisEvents|InputAxisMoveRight
  (params (AxisValue :type Float%20%28single-precision%29))
  ;[1 1 1] Basic Input
  (Pawn|Input|AddMovementInput (Math|Vector|GetRightVector (Math|Rotator|MakeRotator 0.0 0.0 (.yaw (Pawn|GetControlRotation :!class /Script/Engine.Pawn)))) AxisValue false))

(event Input|AxisEvents|InputAxisLookUp
  (params (AxisValue :type Float%20%28single-precision%29))
  ;[1 1 1] Basic Input
  (Pawn|Input|AddControllerPitchInput AxisValue))

(event Input|AxisEvents|InputAxisTurn
  (params (AxisValue :type Float%20%28single-precision%29))
  ;[1 1 1] Basic Input
  (Pawn|Input|AddControllerYawInput AxisValue))

(event Input|MouseEvents|RightMouseButton
  (params (Key :type Key%20Structure))
  ;[1 1 1] Equip Weapon
  (:Pressed
    (if (not (Variables|Default|GetWeapon%20Equip))
      (CallFunction|EquipWeapon true)
      (else
        (CallFunction|EquipWeapon false)))))

(event Input|MouseEvents|LeftMouseButton
  (params (Key :type Key%20Structure))
  (:Pressed
    (if (Variables|Default|GetWeapon%20Equip)
      (Variables|Default|SetShooting true)
      (CallFunction|Shoot (Variables|Default|GetCamera) :!label _label)
      (Utilities|FlowControl|Delay 0.2)
      (if (Variables|Default|GetShooting)
        (goto _label))))
  (:Released
    (Variables|Default|SetShooting false)))

(fn ConstructionScript)

(fn EquipWeapon
  (params (Equip :type Boolean))
  (bind _output_get (Variables|Default|SetWeapon%20Equip Equip))
  (Animation|PlayAnimMontage "/Game/GameContent/RifleAnimSetPro/EquipRifle_Montage.EquipRifle_Montage" 1.0 "None")
  (if _output_get
    (Transformation|AttachComponentToComponent (Variables|Default|GetGun) (Variables|Character|GetMesh) "Rifle" "SnapToTarget" "SnapToTarget" "SnapToTarget" true)
    (Variables|Default|SetbUseControllerRotationYaw true)
    (else
      (Transformation|AttachComponentToComponent (Variables|Default|GetGun) (Variables|Character|GetMesh) "Gun Back" "SnapToTarget" "SnapToTarget" "SnapToTarget" true)
      (Variables|Default|SetbUseControllerRotationYaw false))))

(fn GetAimRotation
  (bind _returnvalue (Pawn|GetControlRotation :!class /Script/Engine.Pawn))
  (if (Pawn|IsPlayerControlled)
    (return (Math|Rotator|MakeRotator (/ (Math|Rotator|NormalizeAxis (- 0.0 (.pitch _returnvalue))) 3.0) 0.0 (/ (Math|Rotator|NormalizeAxis (- (.yaw _returnvalue) (.yaw (Transformation|GetActorRotation)))) 3.0)))
    (elif (Variables|Default|GetPlayer%20in%20sight)
      (return (Math|Rotator|MakeRotator (/ (.Roll (Math|Rotator|BreakRotator (Math|Rotator|FindLookatRotation (Transformation|GetActorLocation) (Transformation|GetActorLocation (Game|Player|GetPlayerPawn 0))))) 3.0) 0.0 0.0)))))

(fn Shoot
  (params (Line%20Start%20Positon :type Scene%20Component%20Object%20Reference))
  (bind _gun (Variables|Default|GetGun))
  (bind _returnvalue (Transformation|GetSocketLocation _gun "Muzzle"))
  (LocalVariables|SetLine%20Start%20Position%20Loco Line%20Start%20Positon)
  (bind (_outhit _returnvalue_2) (Collision|LineTraceByChannel (Transformation|GetSocketLocation (Variables|Default|GetGun) "Muzzle") (select (Pawn|IsPlayerControlled) (+ (Transformation|GetWorldLocation (LocalVariables|GetLine%20Start%20Position%20Loco)) (* (Math|Vector|GetForwardVector (LocalVariables|GetLine%20Start%20Position%20Loco)) 9999.0)) (+ (Transformation|GetActorLocation (Game|Player|GetPlayerPawn 0)) (Math|Vector|MakeVector (Math|Random|RandomFloatinRange -1e+02 1e+02) (Math|Random|RandomFloatinRange -1e+02 1e+02) (Math|Random|RandomFloatinRange -1e+02 1e+02)))) "TraceTypeQuery1" false 0 "None"))
  (bind _returnvalue_3 (Game|SpawnActorfromClass "/Game/Blueprints/GunBlueprint/BulletBase_BP.BulletBase_BP_C" (Math|Transform|MakeTransform _returnvalue (Math|Rotator|FindLookatRotation _returnvalue (select _returnvalue_2 (.ImpactPoint (Collision|BreakHitResult _outhit)) (.TraceEnd (Collision|BreakHitResult _outhit))))) "AlwaysSpawn" 0 1e+01 self self))
  (Audio|PlaySoundatLocation "/Game/GameContent/SciFiWeapLight/Sound/Rifle/Rifle_Fire_Cue.Rifle_Fire_Cue" (Transformation|GetSocketLocation (Variables|Default|GetGun) "Bullet")))