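; Melee enemy AI actor that drives its parent Character through patrol, chase, attack and death.
; Tick spots the player by sphere overlap, angle check and line trace, then chases and plays random attack montages up close.
; Hand and foot spheres attached to mesh sockets deal damage during an interface-set attack window.
; Incoming damage picks hit reactions by exact amount; zero health triggers a knockdown montage, then ragdoll and timed removal.
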(event OnComponentBeginOverlap(HandL)
  (params (OverlappedComponent :type Primitive%20Component%20Object%20Reference) (OtherActor :type Actor%20Object%20Reference) (OtherComp :type Primitive%20Component%20Object%20Reference) (OtherBodyIndex :type Integer) (bFromSweep :type Boolean) (SweepResult :type Hit%20Result%20Structure%20%28by%20ref%29))
  ;[1 1 1] Damage Other Actor
  (if (not (== OtherActor (Variables|Default|GetSelf%20Actor)))
    (if (Variables|Default|GetIs%20Attacking)
      (Game|Damage|ApplyDamage OtherActor (Math|Random|RandomFloatinRange 2.0 5.0) 0 (Variables|Default|GetSelf%20Actor)))))

(event OnComponentBeginOverlap(HandR)
  (params (OverlappedComponent :type Primitive%20Component%20Object%20Reference) (OtherActor :type Actor%20Object%20Reference) (OtherComp :type Primitive%20Component%20Object%20Reference) (OtherBodyIndex :type Integer) (bFromSweep :type Boolean) (SweepResult :type Hit%20Result%20Structure%20%28by%20ref%29))
  ;[1 1 1] Damage Other Actor
  (if (not (== OtherActor (Variables|Default|GetSelf%20Actor)))
    (if (Variables|Default|GetIs%20Attacking)
      (Game|Damage|ApplyDamage OtherActor (Math|Random|RandomFloatinRange 2.0 5.0) 0 (Variables|Default|GetSelf%20Actor)))))

(event OnComponentBeginOverlap(FootL)
  (params (OverlappedComponent :type Primitive%20Component%20Object%20Reference) (OtherActor :type Actor%20Object%20Reference) (OtherComp :type Primitive%20Component%20Object%20Reference) (OtherBodyIndex :type Integer) (bFromSweep :type Boolean) (SweepResult :type Hit%20Result%20Structure%20%28by%20ref%29))
  ;[1 1 1] Damage Other Actor
  (if (not (== OtherActor (Variables|Default|GetSelf%20Actor)))
    (if (Variables|Default|GetIs%20Attacking)
      (Game|Damage|ApplyDamage OtherActor (Math|Random|RandomFloatinRange 5.0 1e+01) 0 (Variables|Default|GetSelf%20Actor)))))

(event OnComponentBeginOverlap(FootR)
  (params (OverlappedComponent :type Primitive%20Component%20Object%20Reference) (OtherActor :type Actor%20Object%20Reference) (OtherComp :type Primitive%20Component%20Object%20Reference) (OtherBodyIndex :type Integer) (bFromSweep :type Boolean) (SweepResult :type Hit%20Result%20Structure%20%28by%20ref%29))
  ;[1 1 1] Damage Other Actor
  (if (not (== OtherActor (Variables|Default|GetSelf%20Actor)))
    (if (Variables|Default|GetIs%20Attacking)
      (Game|Damage|ApplyDamage OtherActor (Math|Random|RandomFloatinRange 5.0 1e+01) 0 (Variables|Default|GetSelf%20Actor)))))

(event Custom|Petrolling
  ;[1 1 1] Petrol
  (bind _output_get (Variables|Default|SetMove%20To%20Loc (.RandomLocation (Class|NavigationSystem|GetRandomPointinNavigableRadius (Transformation|GetActorLocation (Variables|Default|GetSelf%20Actor)) (Variables|Default|GetNav%20Radius)))))
  (AI|AIMoveTo (Variables|Default|GetSelf%20Actor) _output_get 0 5.0 false
    (:OnSuccess
      (Utilities|FlowControl|Delay (Math|Random|RandomFloatinRange 1.0 5.0))
      (CallFunction|Petrolling))))

(event Custom|Go%20to%20Player
  ;[1 1 1] Follow Player
  (if (Variables|Default|GetCan%20See%20Player)
    (Transformation|SetActorRotation (Math|Rotator|FindLookatRotation (Transformation|GetActorLocation) (Transformation|GetActorLocation (Game|Player|GetPlayerPawn 0))))
    (AI|AIMoveTo (Variables|Default|GetSelf%20Actor) "0, 0, 0" (Game|Player|GetPlayerPawn 0) (Math|Random|RandomFloatinRange 1e+02 1.5e+02) false)))

(event Custom|Event%20Take%20Damage
  (params (DamagedActor :type Actor%20Object%20Reference) (Damage :type Float%20%28single-precision%29) (DamageType :type Damage%20Type%20Object%20Reference) (InstigatedBy :type Controller%20Object%20Reference) (DamageCauser :type Actor%20Object%20Reference))
  (bind _self_actor (Variables|Default|GetSelf%20Actor))
  (bind _self_actor_2 (Variables|Default|GetSelf%20Actor))
  (bind _mesh (Variables|/Script/Engine.Character|GetMesh _self_actor))
  (bind _mesh_2 (Variables|/Script/Engine.Character|GetMesh _self_actor_2))
  ;[1 1 1] Getting Damaged
  (Utilities|FlowControl|Sequence
    (:then_0
      ;[1 1 1] Decreas Health
      (bind _output_get (Variables|Default|SetHealth (- (Variables|Default|GetHealth) Damage)))
      (if (<= _output_get 0.0)
        (Variables|Default|SetIs%20Alive false)
        (CallFunction|Death)))
    (:then_1
      (if (== Damage 4.0)
        (Variables|Default|SetGetting%20Hit true)
        (Animation|Montage|PlayMontage _mesh_2 "/Game/GameContent/Animations/FightAnimSetPro/Montage/KB_Hit_p_HighLeft_Weak_Montage.KB_Hit_p_HighLeft_Weak_Montage"
          (:OnCompleted
            _)
          (:OnInterrupted
            _))
        (Utilities|FlowControl|Delay 1.0)
        (Variables|Default|SetGetting%20Hit false)))
    (:then_2
      (if (== Damage 6.0)
        (Variables|Default|SetGetting%20Hit true)
        (Animation|Montage|PlayMontage _mesh_2 "/Game/GameContent/Animations/FightAnimSetPro/Montage/KB_Hit_p_HighRight_Weak_Montage.KB_Hit_p_HighRight_Weak_Montage"
          (:OnCompleted
            _)
          (:OnInterrupted
            _))
        (Utilities|FlowControl|Delay 1.0)
        (Variables|Default|SetGetting%20Hit false)))
    (:then_3
      (if (== Damage 1e+01)
        (Variables|Default|SetGetting%20Hit true)
        (Animation|Montage|PlayMontage _mesh "/Game/GameContent/Animations/FightAnimSetPro/Montage/KB_Hit_m_MidLeft_Med_Montage.KB_Hit_m_MidLeft_Med_Montage"
          (:OnCompleted
            _)
          (:OnInterrupted
            _))
        (Utilities|FlowControl|Delay 1.0)
        (Variables|Default|SetGetting%20Hit false)))
    (:then_4
      (if (== Damage 12.0)
        (Variables|Default|SetGetting%20Hit true)
        (Animation|Montage|PlayMontage _mesh "/Game/GameContent/Animations/FightAnimSetPro/Montage/KB_Hit_m_MidRight_Med_Montage.KB_Hit_m_MidRight_Med_Montage"
          (:OnCompleted
            _)
          (:OnInterrupted
            _))
        (Utilities|FlowControl|Delay 1.0)
        (Variables|Default|SetGetting%20Hit false)))))

(event Custom|Look%20For%20Player
  (bind _self_actor (Variables|Default|GetSelf%20Actor))
  (bind _charactermovement (Variables|/Script/Engine.Character|GetCharacterMovement _self_actor))
  ;[1 1 1] Look for Player
  (if (Collision|IsOverlappingActor (Variables|Default|GetSphere) (Game|GetPlayerCharacter 0) :!class /Script/Engine.PrimitiveComponent)
    (if (> (Class|KismetMathLibrary|DegAcos (Math|Vector|DotProduct (Math|Vector|Normalize (- (Transformation|GetActorLocation (Variables|Default|GetSelf%20Actor)) (Transformation|GetActorLocation (Game|GetPlayerCharacter 0)))) (Transformation|GetActorForwardVector (Variables|Default|GetSelf%20Actor)))) 55.0)
      (bind _outhit (Collision|LineTraceByChannel (Transformation|GetActorLocation (Variables|Default|GetSelf%20Actor)) (Transformation|GetActorLocation (Game|GetPlayerCharacter 0)) "TraceTypeQuery2" true (Utilities|Array|MakeArray (Variables|Default|GetSelf%20Actor)) "None"))
      (if (== (.HitActor (Collision|BreakHitResult _outhit)) (Game|GetPlayerCharacter 0))
        (Variables|Default|SetCan%20See%20Player true)
        (if (> (Transformation|GetDistanceTo (Game|Player|GetPlayerPawn 0)) 3e+02)
          (Variables|/Script/Engine.CharacterMovementComponent|SetMaxWalkSpeed _charactermovement 2.7e+02)
          (else
            (Variables|/Script/Engine.CharacterMovementComponent|SetMaxWalkSpeed _charactermovement 135.0)))
        (else
          (Variables|Default|SetCan%20See%20Player false))))))

(event Custom|Death
  (bind _self_actor (Variables|Default|GetSelf%20Actor))
  (bind _mesh (Variables|/Script/Engine.Character|GetMesh _self_actor))
  ;[1 1 1] Death
  (Animation|Montage|PlayMontage _mesh "/Game/GameContent/Animations/FrankFight/Montage/17_Frank_Hit_KnockDown_Montage.17_Frank_Hit_KnockDown_Montage"
    (:then
      (Utilities|FlowControl|Delay 0.6)
      (Physics|SetSimulatePhysics _mesh true)
      (Collision|SetCollisionEnabled (Variables|/Script/Engine.Character|GetCapsuleComponent _self_actor) "NoCollision")
      (Actor|SetLifeSpan (Variables|Default|GetSelf%20Actor) 1.0))))

(event Custom|Attack%20Player
  (bind _returnvalue (Game|GetPlayerCharacter 0))
  (bind _self_actor (Variables|Default|GetSelf%20Actor))
  (bind _attack_montage (Variables|Default|GetAttack%20Montage))
  (bind _self_actor_2 (Variables|Default|GetSelf%20Actor))
  (bind _returnvalue_2 (Transformation|GetActorLocation _self_actor))
  (bind _returnvalue_3 (Transformation|GetActorLocation _returnvalue))
  (bind _returnvalue_4 (Transformation|GetActorRotation _self_actor_2))
  ;[1 1 1] Attack Player
  (if (Variables|Default|GetCan%20See%20Player)
    (Transformation|SetActorRotation (Math|Rotator|MakeRotator (.roll _returnvalue_4) (.pitch _returnvalue_4) (.yaw (Math|Rotator|FindLookatRotation _returnvalue_2 _returnvalue_3))))
    (if (not (> (Math|Vector|VectorLength (- _returnvalue_2 _returnvalue_3)) 1.2e+02))
      (if (not (Variables|Default|GetGetting%20Hit))
        (if (not (Variables|Default|GetPlaying%20Attack%20Anims))
          (Variables|Default|SetPlaying%20Attack%20Anims true)
          (Animation|Montage|PlayMontage (Variables|/Script/Engine.Character|GetMesh (Variables|Default|GetSelf%20Actor)) (Utilities|Array|Get(acopy) _attack_montage (Math|Random|RandomIntegerinRange 0 (- (Utilities|Array|Length _attack_montage) 1)))
            (:OnCompleted
              (Utilities|FlowControl|Delay 3.0)
              (Variables|Default|SetPlaying%20Attack%20Anims false))
            (:OnInterrupted
              (Utilities|FlowControl|Delay 5.0)
              (Variables|Default|SetPlaying%20Attack%20Anims false))))))))

(event EventBeginPlay
  ;[1 1 1] Begin Play
  (bind _ascharacter (Utilities|Casting|CastToCharacter (Actor|GetParentActor)))
  (Variables|Default|SetSelf%20Actor _ascharacter)
  (Variables|/Script/Engine.CharacterMovementComponent|SetbAllowPhysicsRotationDuringAnimRootMotion (Variables|/Script/Engine.Character|GetCharacterMovement _ascharacter) false)
  (CallFunction|Petrolling)
  (EventDispatchers|BindEventtoOnTakeAnyDamage (Variables|Default|GetSelf%20Actor) (delegate Custom|Event%20Take%20Damage))
  (CallFunction|AttachSpheretoHand))

(event EventTick
  (params (DeltaSeconds :type Float%20%28single-precision%29))
  (if (Variables|Default|GetIs%20Alive)
    ;[1 1 1] Tick
    (CallFunction|LookforPlayer)
    (CallFunction|AttackPlayer)
    (CallFunction|GotoPlayer)
    (if (Variables|Default|GetCan%20See%20Player)
      (Utilities|FlowControl|DoOnce false :!label _label
        (:Completed
          (CallFunction|Petrolling)))
      (else
        (goto _label Reset)))))

(event EventBPIAttack
  (params (Attacking :type Boolean))
  (Variables|Default|SetIs%20Attacking Attacking)
  (Utilities|FlowControl|Delay 1.0)
  (Variables|Default|SetIs%20Attacking false))

(fn ConstructionScript
  (Components|Sphere|SetSphereRadius (Variables|Default|GetSphere) (Variables|Default|GetSphere%20Radius) true))

(fn AttachSpheretoHand
  (Transformation|AttachComponentToComponent (Variables|Default|GetHand%20L) (Variables|/Script/Engine.Character|GetMesh (Variables|Default|GetSelf%20Actor)) "hand_l" "SnapToTarget" "SnapToTarget" "SnapToTarget" true)
  (Transformation|AttachComponentToComponent (Variables|Default|GetHand%20R) (Variables|/Script/Engine.Character|GetMesh (Variables|Default|GetSelf%20Actor)) "hand_r" "SnapToTarget" "SnapToTarget" "SnapToTarget" true)
  (Transformation|AttachComponentToComponent (Variables|Default|GetFoot%20L) (Variables|/Script/Engine.Character|GetMesh (Variables|Default|GetSelf%20Actor)) "foot_l" "SnapToTarget" "SnapToTarget" "SnapToTarget" true)
  (Transformation|AttachComponentToComponent (Variables|Default|GetFoot%20R) (Variables|/Script/Engine.Character|GetMesh (Variables|Default|GetSelf%20Actor)) "foot_r" "SnapToTarget" "SnapToTarget" "SnapToTarget" true))