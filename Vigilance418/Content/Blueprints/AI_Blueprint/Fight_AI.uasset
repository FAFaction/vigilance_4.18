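; Melee enemy AI character that chases, attacks and can be countered by the player.
; When active and near the player, Tick runs attack logic and a line-of-sight trace that switches between chasing and random navmesh patrol.
; Random AttackMoves entries supply paired attack, counter and hit-reaction montages, with limb overlaps dealing damage.
; Partway through attacks, a countering player is snapped into position; damage activates the enemy or triggers knockdown and ragdoll death.
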(event OnComponentBeginOverlap(ArmL)
  (params (OverlappedComponent :type Primitive%20Component%20Object%20Reference) (OtherActor :type Actor%20Object%20Reference) (OtherComp :type Primitive%20Component%20Object%20Reference) (OtherBodyIndex :type Integer) (bFromSweep :type Boolean) (SweepResult :type Hit%20Result%20Structure%20%28by%20ref%29))
  ;[1 1 1] Hit Logic
  (bind _asplayer_character_bp (Utilities|Casting|CastToPlayer_CharacterBP OtherActor))
  (if (not (Variables|/Game/Blueprints/PlayerBlueprint/Player_CharacterBP.Player_CharacterBP_C|GetHit%20Enemy _asplayer_character_bp))
    (if (not (Variables|Default|GetBeing%20Counter))
      (if (Variables|Default|GetAttacking)
        (if (not (or (Variables|Default|GetHitting%20Player) (Variables|Default|GetBeing%20Hit)))
          (Variables|Default|SetHitting%20Player true)
          (Game|Damage|ApplyDamage _asplayer_character_bp 5.0 0 0)
          (CallFunction|MakePlayetLookatAI)
          (bind _returnvalue (Animation|PlayAnimMontage _asplayer_character_bp (.hitreaction (Utilities|Array|Get(acopy) (Variables|Default|GetAttack%20Moves) (Variables|Default|GetFight%20Moves%20Index))) 1.0 "None"))
          (Utilities|FlowControl|Delay _returnvalue)
          (Utilities|FlowControl|Sequence
            (:then_0
              (Variables|Default|SetHitting%20Player false))))))))

(event OnComponentBeginOverlap(ArmR)
  (params (OverlappedComponent :type Primitive%20Component%20Object%20Reference) (OtherActor :type Actor%20Object%20Reference) (OtherComp :type Primitive%20Component%20Object%20Reference) (OtherBodyIndex :type Integer) (bFromSweep :type Boolean) (SweepResult :type Hit%20Result%20Structure%20%28by%20ref%29))
  ;[1 1 1] Hit Logic
  (bind _asplayer_character_bp (Utilities|Casting|CastToPlayer_CharacterBP OtherActor))
  (if (not (Variables|/Game/Blueprints/PlayerBlueprint/Player_CharacterBP.Player_CharacterBP_C|GetHit%20Enemy _asplayer_character_bp))
    (if (not (Variables|Default|GetBeing%20Counter))
      (if (Variables|Default|GetAttacking)
        (if (not (or (Variables|Default|GetHitting%20Player) (Variables|Default|GetBeing%20Hit)))
          (Variables|Default|SetHitting%20Player true)
          (Game|Damage|ApplyDamage _asplayer_character_bp 5.0 0 0)
          (CallFunction|MakePlayetLookatAI)
          (bind _returnvalue (Animation|PlayAnimMontage _asplayer_character_bp (.hitreaction (Utilities|Array|Get(acopy) (Variables|Default|GetAttack%20Moves) (Variables|Default|GetFight%20Moves%20Index))) 1.0 "None"))
          (Utilities|FlowControl|Delay _returnvalue)
          (Utilities|FlowControl|Sequence
            (:then_0
              (Variables|Default|SetHitting%20Player false))))))))

(event OnComponentBeginOverlap(LegL)
  (params (OverlappedComponent :type Primitive%20Component%20Object%20Reference) (OtherActor :type Actor%20Object%20Reference) (OtherComp :type Primitive%20Component%20Object%20Reference) (OtherBodyIndex :type Integer) (bFromSweep :type Boolean) (SweepResult :type Hit%20Result%20Structure%20%28by%20ref%29))
  ;[1 1 1] Hit Logic
  (bind _asplayer_character_bp (Utilities|Casting|CastToPlayer_CharacterBP OtherActor))
  (if (not (Variables|/Game/Blueprints/PlayerBlueprint/Player_CharacterBP.Player_CharacterBP_C|GetHit%20Enemy _asplayer_character_bp))
    (if (not (Variables|Default|GetBeing%20Counter))
      (if (Variables|Default|GetAttack)
        (if (not (or (Variables|Default|GetHitting%20Player) (Variables|Default|GetBeing%20Hit)))
          (Variables|Default|SetHitting%20Player true)
          (Game|Damage|ApplyDamage _asplayer_character_bp 5.0 0 0)
          (CallFunction|MakePlayetLookatAI)
          (bind _returnvalue (Animation|PlayAnimMontage _asplayer_character_bp (.hitreaction (Utilities|Array|Get(acopy) (Variables|Default|GetAttack%20Moves) (Variables|Default|GetFight%20Moves%20Index))) 1.0 "None"))
          (Utilities|FlowControl|Delay _returnvalue)
          (Utilities|FlowControl|Sequence
            (:then_0
              (Variables|Default|SetHitting%20Player false))))))))

(event OnComponentBeginOverlap(LegR)
  (params (OverlappedComponent :type Primitive%20Component%20Object%20Reference) (OtherActor :type Actor%20Object%20Reference) (OtherComp :type Primitive%20Component%20Object%20Reference) (OtherBodyIndex :type Integer) (bFromSweep :type Boolean) (SweepResult :type Hit%20Result%20Structure%20%28by%20ref%29))
  ;[1 1 1] Hit Logic
  (bind _asplayer_character_bp (Utilities|Casting|CastToPlayer_CharacterBP OtherActor))
  (if (not (Variables|/Game/Blueprints/PlayerBlueprint/Player_CharacterBP.Player_CharacterBP_C|GetHit%20Enemy _asplayer_character_bp))
    (if (not (Variables|Default|GetBeing%20Counter))
      (if (Variables|Default|GetAttack)
        (if (not (or (Variables|Default|GetHitting%20Player) (Variables|Default|GetBeing%20Hit)))
          (Variables|Default|SetHitting%20Player true)
          (Game|Damage|ApplyDamage _asplayer_character_bp 5.0 0 0)
          (CallFunction|MakePlayetLookatAI)
          (bind _returnvalue (Animation|PlayAnimMontage _asplayer_character_bp (.hitreaction (Utilities|Array|Get(acopy) (Variables|Default|GetAttack%20Moves) (Variables|Default|GetFight%20Moves%20Index))) 1.0 "None"))
          (Utilities|FlowControl|Delay _returnvalue)
          (Utilities|FlowControl|Sequence
            (:then_0
              (Variables|Default|SetHitting%20Player false))))))))

(event Custom|Fight
  (bind _player_ref (Variables|Default|GetPlayer%20ref))
  ;[1 1 1] Fight Attack Logic
  (if (Variables|Default|GetIs%20Alive)
    (Utilities|IsValid _player_ref
      (:Is%20Valid
        (Utilities|FlowControl|Delay 0.5)
        (if (< (CallFunction|DistancetoPlayer) 2e+02)
          (if (not (or (Variables|/Game/Blueprints/PlayerBlueprint/Player_CharacterBP.Player_CharacterBP_C|GetHit%20Enemy _player_ref) (Variables|/Game/Blueprints/PlayerBlueprint/Player_CharacterBP.Player_CharacterBP_C|GetBeing%20Hit _player_ref)))
            (if (not (or (Variables|Default|GetBeing%20Counter) (Variables|Default|GetBeing%20Hit)))
              (if (not (Variables|Default|GetAttack))
                (Variables|Default|SetAttack true)
                (Variables|Default|SetFight%20Moves%20Index (Math|Random|RandomIntegerinRange 0 (- (Utilities|Array|Length (Variables|Default|GetAttack%20Moves)) 1)))
                (Transformation|SetActorLocationAndRotation (Transformation|GetActorLocation) (Math|Rotator|MakeRotator 0.0 0.0 (.Yaw (Math|Rotator|BreakRotator (Math|Rotator|FindLookatRotation (Transformation|GetActorLocation) (Transformation|GetActorLocation (Game|Player|GetPlayerPawn 0)))))))
                (bind _returnvalue (Animation|PlayAnimMontage (.attack (Utilities|Array|Get(acopy) (Variables|Default|GetAttack%20Moves) (Variables|Default|GetFight%20Moves%20Index))) 1.0 "None"))
                (Utilities|FlowControl|Sequence
                  (:then_2
                    (Utilities|FlowControl|Delay _returnvalue)
                    (Variables|Default|SetAttack false))
                  (:then_3
                    (Utilities|FlowControl|Delay (* _returnvalue 0.3))
                    (CallFunction|BeingCounterbyPlayer)))))))))))

(event Custom|Move%20to%20Player
  (AI|AIMoveTo self (Transformation|GetActorLocation (Game|Player|GetPlayerPawn 0)) 0 1.5e+02 false))

(event Custom|Death
  ;[1 1 1] Damage & Death
  (Animation|Montage|PlayMontage (Variables|Character|GetMesh) "/Game/GameContent/Animations/FrankFight/Montage/17_Frank_Hit_KnockDown_Montage.17_Frank_Hit_KnockDown_Montage" :!label _label
    (:OnBlendOut
      (Physics|SetSimulatePhysics (Variables|Character|GetMesh) true)
      (Collision|SetCollisionEnabled (Variables|Collision|GetCapsuleComponent) "NoCollision")
      (Actor|SetLifeSpan 5.0))
    (:OnInterrupted
      (Utilities|FlowControl|Delay 0.2)
      (goto _label))))

(event Custom|MoveToRandom%20locations
  ;[1 1 1] Petrolling
  (bind _output_get (Variables|Default|SetMoveTo%20Loc (.RandomLocation (Class|NavigationSystem|GetRandomPointinNavigableRadius (Transformation|GetActorLocation) 5e+03))))
  (AI|AIMoveTo self _output_get 0 5.0 false
    (:OnSuccess
      (Utilities|FlowControl|Delay 2.0)
      (CallFunction|MovetoRandomLocations))))

(event Custom|Being%20Counter%20By%20Player
  (bind _player_ref (Variables|Default|GetPlayer%20ref))
  (bind _attack_moves (Variables|Default|GetAttack%20Moves))
  (bind _fight_moves_index (Variables|Default|GetFight%20Moves%20Index))
  (bind _player_ref_2 (Variables|Default|GetPlayer%20ref))
  (bind _returnvalue (Transformation|GetActorRotation _player_ref))
  (bind _output (Utilities|Array|Get(acopy) _attack_moves _fight_moves_index))
  ;[1 1 1] Being Counter By Player
  (bind _asplayer_character_bp (Utilities|Casting|CastToPlayer_CharacterBP (Game|Player|GetPlayerPawn 0)))
  (if (Variables|/Game/Blueprints/PlayerBlueprint/Player_CharacterBP.Player_CharacterBP_C|GetCounter _asplayer_character_bp)
    (Utilities|FlowControl|Sequence
      (:then_0
        (Components|MoveComponentTo (Variables|/Script/Engine.Character|GetCapsuleComponent (Variables|Default|GetPlayer%20ref)) (+ (Transformation|GetActorLocation) (* (Transformation|GetActorForwardVector) (.distance _output))) (Math|Rotator|MakeRotator (.roll _returnvalue) (.pitch _returnvalue) (+ (.yaw (Transformation|GetActorRotation)) 1.8e+02)) true false 0.1 true))
      (:then_1
        (Variables|Default|SetBeing%20Counter true)
        (Variables|/Game/Blueprints/PlayerBlueprint/Player_CharacterBP.Player_CharacterBP_C|SetCountering _player_ref_2 true)
        (bind _returnvalue_2 (Animation|PlayAnimMontage _player_ref_2 (.counter _output) 1.0 "None"))
        (Utilities|FlowControl|Delay _returnvalue_2)
        (Variables|Default|SetBeing%20Counter false)
        (Variables|/Game/Blueprints/PlayerBlueprint/Player_CharacterBP.Player_CharacterBP_C|SetCountering (Variables|Default|GetPlayer%20ref) false)
        (Utilities|FlowControl|Delay 2.0)))))

(event Custom|Hit%20Player
  (params (Hit :type Boolean))
  (Variables|Default|SetAttacking Hit))

(event EventTick
  (params (DeltaSeconds :type Float%20%28single-precision%29))
  (Utilities|FlowControl|Sequence
    (:then_0
      (bind _ashighlighted_bp (Utilities|Casting|CastToHighlighted_BP (Variables|/Script/Engine.ChildActorComponent|GetChildActor (Variables|Default|GetHighlighted))))
      (Class|BPIHightlight|Highlight(Message) _ashighlighted_bp (Variables|Default|GetAttack)))
    (:then_1
      ;[1 1 1] Tick
      (if (Variables|Default|GetIs%20Active)
        (if (< (CallFunction|DistancetoPlayer) 5e+02)
          (CallFunction|Fight)
          (bind _see_player__ (CallFunction|CanSeePlayer))
          (bind _output_get (Variables|Default|SetSee%20Player _see_player__))
          (if _output_get
            (Utilities|FlowControl|Sequence
              (:then_0
                (CallFunction|MovetoPlayer))
              (:then_1
                (goto _label Reset)))
            (else
              (Utilities|FlowControl|DoOnce false :!label _label
                (:Completed
                  (CallFunction|MovetoRandomLocations))))))))))

(event EventBeginPlay
  (bind _asplayer_character_bp (Utilities|Casting|CastToPlayer_CharacterBP (Game|Player|GetPlayerPawn 0)))
  (Variables|Default|SetPlayer%20ref _asplayer_character_bp))

(event Game|Damage|EventAnyDamage
  (params (Damage :type Float%20%28single-precision%29) (DamageType :type Damage%20Type%20Object%20Reference) (InstigatedBy :type Controller%20Object%20Reference) (DamageCauser :type Actor%20Object%20Reference))
  ;[1 1 1] Damage & Death
  (bind _output_get (Variables|Default|SetHealth (- (Variables|Default|GetHealth) Damage)))
  (if (> _output_get 0.0)
    (Variables|Default|SetBeing%20Hit true)
    (Variables|Default|SetIs%20Active true)
    (Utilities|FlowControl|Delay 5.0)
    (Variables|Default|SetBeing%20Hit false)
    (else
      (Variables|Default|SetIs%20Alive false)
      (CallFunction|Death))))

(fn ConstructionScript)

(fn RotationtoPlayer
  (bind _returnvalue (Transformation|GetActorRotation))
  (return (Math|Rotator|MakeRotator (.roll _returnvalue) (.pitch _returnvalue) (.yaw (Math|Rotator|FindLookatRotation (Transformation|GetActorLocation) (Transformation|GetActorLocation (Game|Player|GetPlayerPawn 0)))))))

(fn DistancetoPlayer
  (return (Transformation|GetDistanceTo (Game|Player|GetPlayerPawn 0))))

(fn CanSeePlayer
  (if (< (CallFunction|DistancetoPlayer) 1e+03)
    (bind (_outhit _returnvalue) (Collision|LineTraceByChannel (Transformation|GetActorLocation) (Transformation|GetActorLocation (Game|Player|GetPlayerPawn 0)) "TraceTypeQuery2" true 0 "None"))
    (if _returnvalue
      (Utilities|IsValid (.HitActor (Collision|BreakHitResult _outhit))
        (:Is%20Valid
          (Utilities|Casting|CastToPlayer_CharacterBP (.HitActor (Collision|BreakHitResult _outhit))
            (:then
              (return true))
            (:CastFailed
              _)))
        (:Is%20Not%20Valid
          _))))
  (return false))

(fn MakePlayetLookatAI
  (bind _returnvalue (Game|Player|GetPlayerPawn 0))
  (bind _returnvalue_2 (Transformation|GetActorRotation _returnvalue))
  (Transformation|SetActorRotation _returnvalue (Math|Rotator|MakeRotator (.roll _returnvalue_2) (.pitch _returnvalue_2) (.yaw (Math|Rotator|FindLookatRotation (Transformation|GetActorLocation _returnvalue) (Transformation|GetActorLocation)))) true))