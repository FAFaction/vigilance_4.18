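; AI path Blueprint that defines an array of move points from a spline laid out in the level.
; The construction script clears and rebuilds MovePoints from the spline point locations, stored in local rather than world space.
; It adds a text component showing the loop index at each location, sampled at index minus one, so labels are offset from spline indices.
; The event graph has no active logic.
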(event EventBeginPlay)

(event Collision|EventActorBeginOverlap
  (params (OtherActor :type Actor%20Object%20Reference)))

(event EventTick
  (params (DeltaSeconds :type Float%20%28single-precision%29)))

(fn ConstructionScript
  (bind _spline (Variables|Default|GetSpline))
  (Utilities|Array|Clear (Variables|Default|GetMove%20Points))
  (for _index (range 0 (Spline|GetNumberOfSplinePoints _spline))
    (bind _returnvalue (AddComponent|AddTextRenderComponent false (Math|Transform|MakeTransform (Spline|GetLocationatSplinePoint _spline (- _index 1) "Local"))))
    (Rendering|Components|TextRender|SetText _returnvalue (Utilities|Text|ToText(Integer) _index))
    (Utilities|Array|Add (Variables|Default|GetMove%20Points) (Spline|GetLocationatSplinePoint _spline (- _index 1) "Local"))))