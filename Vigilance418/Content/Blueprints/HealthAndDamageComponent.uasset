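; Health component that handles damage, directional hit reactions and death for its owning Character.
; It binds to the owner's TakeAnyDamage and subtracts from Health whenever the damage causer is valid.
; Survivors play a front, back, left or right montage from the raw, unnormalized yaw difference to the causer, in three damage-based strengths.
; At zero health the mesh ragdolls, a fall sound plays, then OnDeath fires and the character is destroyed.
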(event Custom|On%20Take%20Damage
  (params (DamagedActor :type Actor%20Object%20Reference) (Damage :type Float%20%28single-precision%29) (DamageType :type Damage%20Type%20Object%20Reference) (InstigatedBy :type Controller%20Object%20Reference) (DamageCauser :type Actor%20Object%20Reference))
  (Utilities|IsValid DamageCauser
    (:Is%20Valid
      (Variables|Default|SetDamage Damage)
      (Variables|Default|SetDamage%20Causer DamageCauser)
      (bind _output_get (Variables|Default|SetHealth (- (Variables|Default|GetHealth) Damage)))
      (if (<= _output_get 0.0)
        (bind _ascharacter (Utilities|Casting|CastToCharacter DamagedActor))
        (Collision|SetCollisionEnabled (Variables|/Script/Engine.Character|GetMesh _ascharacter) "QueryAndPhysics")
        (Physics|SetSimulatePhysics (Variables|/Script/Engine.Character|GetMesh _ascharacter) true)
        (Collision|SetCollisionEnabled (Variables|/Script/Engine.Character|GetCapsuleComponent _ascharacter) "NoCollision")
        (Utilities|FlowControl|Delay 0.3)
        (Audio|PlaySoundatLocation "/Game/GameContent/Punch_Fighting_SFX/Wavs/Body_Fall/Body_Fall_1_Cue.Body_Fall_1_Cue" (Transformation|GetActorLocation (Components|GetOwner)))
        (Utilities|FlowControl|Delay 4.0)
        (Default|CallOnDeath)
        (Actor|DestroyActor _ascharacter)
        (else
          (CallFunction|React DamageCauser)
          (bind _ascharacter_2 (Utilities|Casting|CastToCharacter (Components|GetOwner)))
          (Variables|Default|SetOwner%20Character _ascharacter_2)
          (if (> (- (.yaw (Transformation|GetActorRotation (Components|GetOwner))) (.yaw (Transformation|GetActorRotation (stale Custom|React Damage%20Causer)))) 0.0)
            (if (> (- (.yaw (Transformation|GetActorRotation (Components|GetOwner))) (.yaw (Transformation|GetActorRotation (stale Custom|React Damage%20Causer)))) 1.3e+02)
              (if (> (Variables|Default|GetDamage) 1e+01) :!label _label
                (Animation|PlayAnimMontage (Variables|Default|GetOwner%20Character) "/Game/GameContent/Animations/FightAnimSetPro/Montage/KB_Hit_m_HighFront_Stagger_Montage.KB_Hit_m_HighFront_Stagger_Montage" 1.0 "None")
                (elif (> (Variables|Default|GetDamage) 5.0)
                  (Animation|PlayAnimMontage (Variables|Default|GetOwner%20Character) "/Game/GameContent/Animations/FightAnimSetPro/Montage/KB_Hit_m_HighFront_Med_Montage.KB_Hit_m_HighFront_Med_Montage" 1.0 "None")
                  (else
                    (Animation|PlayAnimMontage (Variables|Default|GetOwner%20Character) "/Game/GameContent/Animations/FightAnimSetPro/Montage/KB_Hit_m_HighFront_Weak_Montage.KB_Hit_m_HighFront_Weak_Montage" 1.0 "None"))))
              (elif (> (- (.yaw (Transformation|GetActorRotation (Components|GetOwner))) (.yaw (Transformation|GetActorRotation (stale Custom|React Damage%20Causer)))) 45.0)
                (if (> (Variables|Default|GetDamage) 1e+01)
                  (Animation|PlayAnimMontage (Variables|Default|GetOwner%20Character) "/Game/GameContent/Animations/FightAnimSetPro/Montage/KB_Hit_m_MidRight_Stagger_Montage.KB_Hit_m_MidRight_Stagger_Montage" 1.0 "None")
                  (elif (> (Variables|Default|GetDamage) 5.0)
                    (Animation|PlayAnimMontage (Variables|Default|GetOwner%20Character) "/Game/GameContent/Animations/FightAnimSetPro/Montage/KB_Hit_m_MidRight_Med_Montage.KB_Hit_m_MidRight_Med_Montage" 1.0 "None")
                    (else
                      (Animation|PlayAnimMontage (Variables|Default|GetOwner%20Character) "/Game/GameContent/Animations/FightAnimSetPro/Montage/KB_Hit_p_HighRight_Weak_Montage.KB_Hit_p_HighRight_Weak_Montage" 1.0 "None"))))
                (else
                  (if (> (Variables|Default|GetDamage) 1e+01) :!label _label_2
                    (Animation|PlayAnimMontage (Variables|Default|GetOwner%20Character) "/Game/GameContent/Animations/FightAnimSetPro/Montage/KB_Hit_m_HighBack_Stagger_Montage.KB_Hit_m_HighBack_Stagger_Montage" 1.0 "None")
                    (elif (> (Variables|Default|GetDamage) 5.0)
                      (Animation|PlayAnimMontage (Variables|Default|GetOwner%20Character) "/Game/GameContent/Animations/FightAnimSetPro/Montage/KB_Hit_m_MidBack_Med_Montage.KB_Hit_m_MidBack_Med_Montage" 1.0 "None")
                      (else
                        (Animation|PlayAnimMontage (Variables|Default|GetOwner%20Character) "/Game/GameContent/Animations/FightAnimSetPro/Montage/KB_Hit_m_HighBack_Weak_Montage.KB_Hit_m_HighBack_Weak_Montage" 1.0 "None")))))))
            (elif (< (- (.yaw (Transformation|GetActorRotation (Components|GetOwner))) (.yaw (Transformation|GetActorRotation (stale Custom|React Damage%20Causer)))) -1.3e+02)
              (goto _label)
              (elif (< (- (.yaw (Transformation|GetActorRotation (Components|GetOwner))) (.yaw (Transformation|GetActorRotation (stale Custom|React Damage%20Causer)))) -45.0)
                (if (> (Variables|Default|GetDamage) 1e+01)
                  (Animation|PlayAnimMontage (Variables|Default|GetOwner%20Character) "/Game/GameContent/Animations/FightAnimSetPro/Montage/KB_Hit_m_MidLeft_Stagger_Montage.KB_Hit_m_MidLeft_Stagger_Montage" 1.0 "None")
                  (elif (> (Variables|Default|GetDamage) 5.0)
                    (Animation|PlayAnimMontage (Variables|Default|GetOwner%20Character) "/Game/GameContent/Animations/FightAnimSetPro/Montage/KB_Hit_m_MidLeft_Med_Montage.KB_Hit_m_MidLeft_Med_Montage" 1.0 "None")
                    (else
                      (Animation|PlayAnimMontage (Variables|Default|GetOwner%20Character) "/Game/GameContent/Animations/FightAnimSetPro/Montage/KB_Hit_m_MidLeft_Weak_Montage.KB_Hit_m_MidLeft_Weak_Montage" 1.0 "None"))))
                (else
                  (goto _label_2))))))))))

(event Custom|React
  (params (Damage%20Causer :type Actor%20Object%20Reference))
  (bind _returnvalue (Components|GetOwner))
  (bind _returnvalue_2 (Transformation|GetActorRotation Damage%20Causer))
  (bind _damage (Variables|Default|GetDamage))
  (bind _returnvalue_3 (> _damage 5.0))
  (bind _returnvalue_4 (> _damage 1e+01))
  (bind _returnvalue_5 (Transformation|GetActorRotation _returnvalue))
  (bind _returnvalue_6 (- (.yaw _returnvalue_5) (.yaw _returnvalue_2)))
  (bind _ascharacter (Utilities|Casting|CastToCharacter (Components|GetOwner)))
  (Variables|Default|SetOwner%20Character _ascharacter)
  (if (> _returnvalue_6 0.0)
    (if (> _returnvalue_6 1.3e+02)
      (if _returnvalue_4 :!label _label
        (Animation|PlayAnimMontage (Variables|Default|GetOwner%20Character) "/Game/GameContent/Animations/FightAnimSetPro/Montage/KB_Hit_m_HighFront_Stagger_Montage.KB_Hit_m_HighFront_Stagger_Montage" 1.0 "None")
        (elif _returnvalue_3
          (Animation|PlayAnimMontage (Variables|Default|GetOwner%20Character) "/Game/GameContent/Animations/FightAnimSetPro/Montage/KB_Hit_m_HighFront_Med_Montage.KB_Hit_m_HighFront_Med_Montage" 1.0 "None")
          (else
            (Animation|PlayAnimMontage (Variables|Default|GetOwner%20Character) "/Game/GameContent/Animations/FightAnimSetPro/Montage/KB_Hit_m_HighFront_Weak_Montage.KB_Hit_m_HighFront_Weak_Montage" 1.0 "None"))))
      (elif (> _returnvalue_6 45.0)
        (if _returnvalue_4
          (Animation|PlayAnimMontage (Variables|Default|GetOwner%20Character) "/Game/GameContent/Animations/FightAnimSetPro/Montage/KB_Hit_m_MidRight_Stagger_Montage.KB_Hit_m_MidRight_Stagger_Montage" 1.0 "None")
          (elif _returnvalue_3
            (Animation|PlayAnimMontage (Variables|Default|GetOwner%20Character) "/Game/GameContent/Animations/FightAnimSetPro/Montage/KB_Hit_m_MidRight_Med_Montage.KB_Hit_m_MidRight_Med_Montage" 1.0 "None")
            (else
              (Animation|PlayAnimMontage (Variables|Default|GetOwner%20Character) "/Game/GameContent/Animations/FightAnimSetPro/Montage/KB_Hit_p_HighRight_Weak_Montage.KB_Hit_p_HighRight_Weak_Montage" 1.0 "None"))))
        (else
          (if _returnvalue_4 :!label _label_2
            (Animation|PlayAnimMontage (Variables|Default|GetOwner%20Character) "/Game/GameContent/Animations/FightAnimSetPro/Montage/KB_Hit_m_HighBack_Stagger_Montage.KB_Hit_m_HighBack_Stagger_Montage" 1.0 "None")
            (elif _returnvalue_3
              (Animation|PlayAnimMontage (Variables|Default|GetOwner%20Character) "/Game/GameContent/Animations/FightAnimSetPro/Montage/KB_Hit_m_MidBack_Med_Montage.KB_Hit_m_MidBack_Med_Montage" 1.0 "None")
              (else
                (Animation|PlayAnimMontage (Variables|Default|GetOwner%20Character) "/Game/GameContent/Animations/FightAnimSetPro/Montage/KB_Hit_m_HighBack_Weak_Montage.KB_Hit_m_HighBack_Weak_Montage" 1.0 "None")))))))
    (elif (< _returnvalue_6 -1.3e+02)
      (goto _label)
      (elif (< _returnvalue_6 -45.0)
        (if _returnvalue_4
          (Animation|PlayAnimMontage (Variables|Default|GetOwner%20Character) "/Game/GameContent/Animations/FightAnimSetPro/Montage/KB_Hit_m_MidLeft_Stagger_Montage.KB_Hit_m_MidLeft_Stagger_Montage" 1.0 "None")
          (elif _returnvalue_3
            (Animation|PlayAnimMontage (Variables|Default|GetOwner%20Character) "/Game/GameContent/Animations/FightAnimSetPro/Montage/KB_Hit_m_MidLeft_Med_Montage.KB_Hit_m_MidLeft_Med_Montage" 1.0 "None")
            (else
              (Animation|PlayAnimMontage (Variables|Default|GetOwner%20Character) "/Game/GameContent/Animations/FightAnimSetPro/Montage/KB_Hit_m_MidLeft_Weak_Montage.KB_Hit_m_MidLeft_Weak_Montage" 1.0 "None"))))
        (else
          (goto _label_2))))))

(event EventBeginPlay
  (EventDispatchers|BindEventtoOnTakeAnyDamage (Components|GetOwner) (delegate Custom|On%20Take%20Damage)))