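; Checkpoint trigger actor that records the player's checkpoint and location in the game instance.
; When Player_CharacterBP overlaps its box, it passes itself and a PlayerLocation offset from the actor's position to GameGI's UpdateCheckpoint, then prints a debug message.
; A DoOnce reset after a short delay throttles repeated updates.
; The construction script sizes the box from the BoxExtend variable.
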(event OnComponentBeginOverlap(Box)
  (params (OverlappedComponent :type Primitive%20Component%20Object%20Reference) (OtherActor :type Actor%20Object%20Reference) (OtherComp :type Primitive%20Component%20Object%20Reference) (OtherBodyIndex :type Integer) (bFromSweep :type Boolean) (SweepResult :type Hit%20Result%20Structure%20%28by%20ref%29))
  (Utilities|Casting|CastToPlayer_CharacterBP OtherActor)
  (Utilities|FlowControl|Sequence
    (:then_0
      (Utilities|FlowControl|DoOnce false :!label _label
        (:Completed
          (bind _asgame_gi (Utilities|Casting|CastToGameGI (Game|GetGameInstance)))
          (Default|UpdateCheckpoint _asgame_gi self (+ (Variables|Default|GetPlayer%20Location) (Transformation|GetActorLocation)))
          (Development|PrintString "Check point Updated" true true "(R=1.000000,G=0.000000,B=0.205652,A=1.000000)"))))
    (:then_1
      (Utilities|FlowControl|Delay 2.0)
      (goto _label Reset))))

(event EventBeginPlay)

(event Collision|EventActorBeginOverlap
  (params (OtherActor :type Actor%20Object%20Reference)))

(event EventTick
  (params (DeltaSeconds :type Float%20%28single-precision%29)))

(fn ConstructionScript
  (Components|Box|SetBoxExtent (Variables|Default|GetBox) (Variables|Default|GetBox%20Extend) true))