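; Mission set-piece actor that stages the execution of Decks by thugs, then sets up the shootout that follows.
; Its trigger gathers enemies around a kneeling Decks, then on player entry plays paired execution montages, spreads the thugs, and swaps Decks for a ragdoll plus VIP_Pass.
; Tick prunes dead enemies, then prompts a search for clues.
; EventGraph also holds a keyed interrogation dialogue whose starting logic is disconnected.
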(event Custom|Start%20Yealling
  ;[1 0 0] For Later
)

(event Custom|Choice%20select
  (params (Interrogate :type Boolean))
  (if Interrogate
    (switch int (Variables|Default|GetQuestion%20Num)
      (:0
        (CallFunction|Question1)
        (Math|Integer|IncrementInt (Variables|Default|GetQuestion%20Num) :!label _label))
      (:1
        (CallFunction|Question2)
        (goto _label))
      (:2
        (CallFunction|Question3)
        (goto _label))
      (:3
        (CallFunction|Question4)))
    (else
      (switch int (Variables|Default|GetQuestion%20Num)
        (:0
          (bind _returnvalue (UserInterface|CreateWidget "/Game/UI/NotificitionUI_WB.NotificitionUI_WB_C" :!label _label_2))
          (Default|ShowNotification _returnvalue "you need to find the bounty location from him" 1.0)
          (UserInterface|Viewport|AddtoViewport _returnvalue 0))
        (:1
          (goto _label_2))
        (:2
          (goto _label_2))
        (:3
          (CallFunction|Leave4))))))

(event Custom|Question%201
  (bind _decks (Variables|Default|GetDecks))
  (bind _mesh (Variables|/Script/Engine.Character|GetMesh _decks))
  ;[1 1 1] Interrogation Question 1
  (Variables|Default|SetSpacking true)
  (Widget|RemovefromParent (Variables|Default|GetChoice%20UI))
  (Utilities|Time|SetGlobalTimeDilation 1.0)
  (Default|CustomAimfromOutside (Variables|Default|GetPlayer) true)
  (Pawn|SetControlRotation (Game|GetPlayerController 0) (Math|Rotator|FindLookatRotation (Transformation|GetActorLocation (Variables|Default|GetPlayer)) (Transformation|GetActorLocation (Variables|Default|GetDecks))))
  (Utilities|FlowControl|Delay 0.2)
  (Transformation|SetActorRotation _decks (Math|Rotator|FindLookatRotation (Transformation|GetActorLocation (Variables|Default|GetDecks)) (Transformation|GetActorLocation (Variables|Default|GetPlayer))))
  (Components|Animation|PlayAnimation _mesh "/Game/GameContent/Animations/FrankFight/14_Frank_Hit_Heavy_Inplace.14_Frank_Hit_Heavy_Inplace" false)
  (Utilities|FlowControl|Delay 0.2)
  (Components|Animation|PlayAnimation _mesh "/Game/GameContent/Animations/MovementAnimSetPro/HandsupPose.HandsupPose" true)
  (Utilities|FlowControl|Delay 0.5)
  (Utilities|Dialogue "Civilian" "Ok ok take what ever you want just don't shoot")
  (Utilities|FlowControl|Delay 2.0)
  (CallFunction|ShowChoiceMenu)
  (Variables|Default|SetSpacking true))

(event Custom|Question%203
  (bind _decks (Variables|Default|GetDecks))
  (bind _mesh (Variables|/Script/Engine.Character|GetMesh _decks))
  ;[1 1 1] Interrogation Question 3
  (Variables|Default|SetSpacking false)
  (Widget|RemovefromParent (Variables|Default|GetChoice%20UI))
  (Utilities|Time|SetGlobalTimeDilation 1.0)
  (Pawn|SetControlRotation (Game|GetPlayerController 0) (Math|Rotator|FindLookatRotation (Transformation|GetActorLocation (Variables|Default|GetPlayer)) (+ (Transformation|GetActorLocation) (Variables|Default|GetShoot%20At%20Loc))))
  (Utilities|FlowControl|Delay 1.0)
  (Default|CustomShootfromOutside (Variables|Default|GetPlayer))
  (Components|Animation|PlayAnimation _mesh "/Game/GameContent/Animations/FightAnimSetPro/KB_Hit_m_LowRight_Med.KB_Hit_m_LowRight_Med" false)
  (Utilities|FlowControl|Delay 1.0)
  (Components|Animation|PlayAnimation _mesh "/Game/GameContent/Animations/MovementAnimSetPro/HandsupPose.HandsupPose" true)
  (Pawn|SetControlRotation (Game|GetPlayerController 0) (Math|Rotator|FindLookatRotation (Transformation|GetActorLocation (Variables|Default|GetPlayer)) (Transformation|GetActorLocation (Variables|Default|GetDecks))))
  (Utilities|Dialogue "Civilian" "Ok ok i will tell you what i know")
  (Utilities|FlowControl|Delay 1.0)
  (Utilities|Dialogue "Civilian" "I saw him with some guys who cummited the murder and they where calling him Boss")
  (Utilities|FlowControl|Delay 2.0)
  (CallFunction|ShowChoiceMenu)
  (Variables|Default|SetSpacking true))

(event Custom|Question%204
  (bind _returnvalue (Game|GetPlayerController 0))
  (bind _player (Variables|Default|GetPlayer))
  ;[1 1 1] Question 4
  (Variables|Default|SetSpacking false)
  (Widget|RemovefromParent (Variables|Default|GetChoice%20UI))
  (Utilities|Time|SetGlobalTimeDilation 1.0)
  (Utilities|FlowControl|Delay 0.5)
  (Utilities|Dialogue "Player" "Ok What do you about the people who cummited the murder ?")
  (Utilities|FlowControl|Delay 2.0)
  (Utilities|Dialogue "Civilian" "Nothing to much")
  (Utilities|FlowControl|Delay 1.0)
  (Utilities|Dialogue "Civilian" "I just saw them a few times hanging out in the 1's Bar")
  (Utilities|FlowControl|Delay 1.0)
  (Utilities|Dialogue "Civilian" "They should be there by now")
  (Utilities|FlowControl|Delay 2.0)
  (bind _asplayer_character_bp (Utilities|Casting|CastToPlayer_CharacterBP (Game|GetPlayerCharacter 0)))
  (Default|ShowNewMissionObjective _asplayer_character_bp "Go to the Bar and find Suspect")
  (bind _returnvalue_2 (UserInterface|CreateWidget "/Game/UI/NotificitionUI_WB.NotificitionUI_WB_C"))
  (Default|ShowNotification _returnvalue_2 "Go to the Bar" 4.0)
  (UserInterface|Viewport|AddtoViewport _returnvalue_2 0)
  (bind _outactors (Actor|GetAllActorsOfClass "/Game/Blueprints/CustomBlueprints/FightAndInterogationInThneBar/WaypointToBar.WaypointToBar_C"))
  (Default|ShowWayPoint (Utilities|Array|Get(acopy) _outactors) true)
  (Input|EnableInput _player _returnvalue)
  (Default|CustomAimfromOutside _player false)
  (Input|DisableInput _returnvalue)
  (bind _asdecks (Utilities|Casting|CastToDecks (Variables|Default|GetDecks)))
  (Rendering|SetVisibility (Variables|/Game/Blueprints/CustomBlueprints/GettingInfoFromPoice/Decks.Decks_C|GetWidget _asdecks) false false)
  (Variables|Default|SetSpacking true)
  (Utilities|Dialogue))

(event Custom|Leave%204
  ;[1 1 1] Leave 4
)

(event Custom|Show%20Choice%20menu
  (bind _returnvalue (UserInterface|CreateWidget "/Game/Blueprints/CustomBlueprints/ShootoutAfterDecksGotKilled/Interrogation_ChoiceUI.Interrogation_ChoiceUI_C"))
  (bind _output_get (Variables|Default|SetChoice%20UI _returnvalue))
  (UserInterface|Viewport|AddtoViewport _output_get 0))

(event Custom|Question%202
  ;[1 1 1] Interrogation Question 2
  (Variables|Default|SetSpacking false)
  (Widget|RemovefromParent (Variables|Default|GetChoice%20UI))
  (Utilities|Time|SetGlobalTimeDilation 1.0)
  (Utilities|Dialogue "Player" "Ok What do you know about the Zeno organization ")
  (Utilities|FlowControl|Delay 2.0)
  (Utilities|Dialogue "Civilian" "I know Absolutely nothing about them I'm just a simple citizen")
  (Utilities|FlowControl|Delay 2.0)
  (CallFunction|ShowChoiceMenu)
  (Variables|Default|SetSpacking true))

(event EventBeginPlay
  (|CallParentFunction)
  (bind _asplayer_character_bp (Utilities|Casting|CastToPlayer_CharacterBP (Game|Player|GetPlayerPawn 0)))
  (Variables|Default|SetPlayer _asplayer_character_bp))

(event Collision|EventActorBeginOverlap
  (params (OtherActor :type Actor%20Object%20Reference))
  (|CallParentFunction OtherActor) ; This node is disabled and will not be called.\nDrag off pins to build functionality.
)

(event EventTick
  (params (DeltaSeconds :type Float%20%28single-precision%29)))

(event EventOnPlayerEnterTrigger)

(event Input|KeyboardEvents|1
  (params (Key :type Key%20Structure))
  (:Pressed
    (if (Variables|Default|GetSpacking)
      (CallFunction|ChoiceSelect false))))

(event Input|KeyboardEvents|2
  (params (Key :type Key%20Structure))
  (:Pressed
    (if (Variables|Default|GetSpacking)
      (CallFunction|ChoiceSelect true))))

(event OnComponentBeginOverlap(Trigger)
  (params (OverlappedComponent :type Primitive%20Component%20Object%20Reference) (OtherActor :type Actor%20Object%20Reference) (OtherComp :type Primitive%20Component%20Object%20Reference) (OtherBodyIndex :type Integer) (bFromSweep :type Boolean) (SweepResult :type Hit%20Result%20Structure%20%28by%20ref%29))
  ;[1 1 1] Trigger
  (bind _asplayer_character_bp (Utilities|Casting|CastToPlayer_CharacterBP OtherActor)
    (:then
      (Variables|Default|SetPlayer _asplayer_character_bp)
      (Utilities|FlowControl|DoOnce false
        (:Completed
          (CallFunction|WhenPlayerClose))))
    (:CastFailed
      (bind _asdecks (Utilities|Casting|CastToDecks OtherActor))
      (Variables|Default|SetDecks _asdecks)
      (Utilities|FlowControl|DoOnce false
        (:Completed
          (CallFunction|WhenDecksEnterTrigger))))))

(event Custom|When%20Decks%20enter%20trigger
  (bind _enemise (Variables|Default|GetEnemise))
  (bind _decks (Variables|Default|GetDecks))
  (bind _decks_2 (Variables|Default|GetDecks))
  ;[0.9367 0.3612 1] Comment
  (Utilities|FlowControl|Delay 2.0)
  (AI|AIMoveTo (Utilities|Array|Get(acopy) (Variables|Default|GetEnemise)) (+ (Transformation|GetActorLocation _decks_2) (* (Transformation|GetActorForwardVector _decks_2) -1e+01)) _decks_2 1e+02 false
    (:OnSuccess
      (for _index (range 1 (- (Utilities|Array|Length _enemise) 1))
        (Utilities|IsValid (Utilities|Array|Get(acopy) _enemise _index)
          (:Is%20Valid
            (AI|AIMoveTo (Utilities|Array|Get(acopy) _enemise _index) "0, 0, 0" (Variables|Default|GetDecks) 2e+02 false))))
      (Transformation|SetActorRotation _decks (Transformation|GetWorldRotation (Variables|Default|GetArrow)))
      (Components|Animation|PlayAnimation (Variables|/Script/Engine.Character|GetMesh _decks) "/Game/GameContent/Animations/Hostage/Idle_HandsUpHostage_Kneel_Loop.Idle_HandsUpHostage_Kneel_Loop" true))))

(event Custom|When%20player%20Close
  (bind _player (Variables|Default|GetPlayer))
  (bind _enemise (Variables|Default|GetEnemise))
  ;[1 1 1] Start shoot out
  (Animation|PlayAnimMontage (Utilities|Array|Get(acopy) (Variables|Default|GetEnemise)) "/Game/GameContent/Animations/Hostage/Montage/Paired_Pistol_HandsUpHostage_Kneel_HeadShotExecution_Att_Montage.Paired_Pistol_HandsUpHostage_Kneel_HeadShotExecution_Att_Montage" 1.0 "None")
  (Animation|PlayAnimMontage (Variables|Default|GetDecks) "/Game/GameContent/Animations/Hostage/Montage/Paired_Pistol_HandsUpHostage_Kneel_HeadShotExecution_Vic_Montage.Paired_Pistol_HandsUpHostage_Kneel_HeadShotExecution_Vic_Montage" 1.0 "None")
  (Utilities|FlowControl|Delay 1.5)
  (Utilities|FlowControl|Sequence
    (:then_0
      (AI|AIMoveTo (Utilities|Array|Get(acopy) (Variables|Default|GetEnemise)) (+ (Transformation|GetActorLocation _player) (* (Transformation|GetActorForwardVector _player) 1e+03)) 0 1e+01 false
        (:OnSuccess
          (Utilities|FlowControl|Delay 1.0)
          (for _index (range 1 (- (Utilities|Array|Length _enemise) 1))
            (bind _asnew_shooter_ai_thug (Utilities|Casting|CastToNewShooterAI_Thug (Utilities|Array|Get(acopy) _enemise _index)))
            (Variables|/Script/Engine.CharacterMovementComponent|SetMaxWalkSpeed (Variables|/Script/Engine.Character|GetCharacterMovement _asnew_shooter_ai_thug) 2.7e+02)
            (Variables|/Game/Blueprints/AI_Blueprint/ShooterAI/NewShooterAI/NewShooterAI.NewShooterAI_C|SetAI%20Sight%20Limit _asnew_shooter_ai_thug 2e+03)
            (AI|AIMoveTo (Utilities|Array|Get(acopy) _enemise _index) (+ (Utilities|Array|Get(acopy) (Variables|Default|GetAI%20Spread%20Locations) _index) (Transformation|GetActorLocation)) 0 5.0 false))
          (Utilities|FlowControl|Delay 5.0)
          (for _array_element (Variables|Default|GetEnemise)
            (Transformation|SetActorRotation _array_element (Math|Rotator|MakeRotator 0.0 0.0 (.yaw (Utilities|RottoPlayer _array_element))))))))
    (:then_1
      ;[1 1 1] Destrioy decks and spawn in dummy and VIP pass
      (bind _returnvalue (Game|SpawnActorfromClass "/Script/Engine.SkeletalMeshActor" (Transformation|GetActorTransform (Variables|Default|GetDecks)) "AdjustIfPossibleButAlwaysSpawn" 0 0))
      (Class|SkinnedMeshComponent|SetSkeletalMesh (Variables|/Script/Engine.SkeletalMeshActor|GetSkeletalMeshComponent _returnvalue) (Variables|/Script/Engine.SkinnedMeshComponent|GetSkeletalMesh (Variables|/Script/Engine.Character|GetMesh (Variables|Default|GetDecks))) true)
      (Collision|SetCollisionEnabled (Variables|/Script/Engine.SkeletalMeshActor|GetSkeletalMeshComponent _returnvalue) "QueryAndPhysics")
      (Physics|SetSimulatePhysics (Variables|/Script/Engine.SkeletalMeshActor|GetSkeletalMeshComponent _returnvalue) true)
      (Game|SpawnActorfromClass "/Game/Blueprints/CustomBlueprints/ShootoutAfterDecksGotKilled/VIP_Pass.VIP_Pass_C" (Math|Transform|MakeTransform (.RandomLocation (Class|NavigationSystem|GetRandomPointinNavigableRadius (Transformation|GetActorLocation (Variables|Default|GetDecks)) 5e+02))) "AdjustIfPossibleButAlwaysSpawn" 0 0)
      (Actor|DestroyActor (Variables|Default|GetDecks)))))

(event EventTick
  (params (DeltaSeconds :type Float%20%28single-precision%29))
  (bind _enemise (Variables|Default|GetEnemise))
  ;[1 1 1] Tick
  (for _array_element _enemise
    (Utilities|IsValid _array_element
      (:Is%20Not%20Valid
        (Utilities|Array|RemoveItem _enemise _array_element))))
  (if (not (> (Utilities|Array|Length _enemise) 0))
    (Utilities|FlowControl|DoOnce false
      (:Completed
        (bind _returnvalue (UserInterface|CreateWidget "/Game/UI/NotificitionUI_WB.NotificitionUI_WB_C"))
        (UserInterface|Viewport|AddtoViewport _returnvalue 0)
        (Default|ShowNotification _returnvalue "Search Decks for clues" 2.0)))))

(fn ConstructionScript
  (|CallParentFunction))