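; Child actor that hosts a hacking UI and hands player control to its parent actor once the hack completes.
; BeginPlay creates a HackUI, sets it on the Widget component and binds Hacked to its done-hacking event.
; Hacked blends the player's view to the parent actor, waits out the blend, hides the widget, then possesses the parent if it is a Pawn.
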(event Custom|Hacked
  (bind _returnvalue (Game|GetPlayerController 0))
  (Game|Player|SetViewTargetwithBlend _returnvalue (Actor|GetParentActor) 0.2 "VTBlend_Cubic" 0.0 false)
  (Utilities|FlowControl|Delay 0.2)
  (Rendering|SetVisibility (Variables|Default|GetWidget) false false)
  (bind _aspawn (Utilities|Casting|CastToPawn (Actor|GetParentActor)))
  (Pawn|Possess _returnvalue _aspawn))

(event EventBeginPlay
  (bind _returnvalue (UserInterface|CreateWidget "/Game/Blueprints/CustomBlueprints/GettingInfoFromPoice/HackUI.HackUI_C"))
  (UserInterface|SetWidget (Variables|Default|GetWidget) _returnvalue)
  (bind _output_get (Variables|Default|SetUI _returnvalue))
  (EventDispatchers|BindEventtoDoneHacking _output_get (delegate Custom|Hacked)))

(event Collision|EventActorBeginOverlap
  (params (OtherActor :type Actor%20Object%20Reference)))

(event EventTick
  (params (DeltaSeconds :type Float%20%28single-precision%29)))

(fn ConstructionScript)