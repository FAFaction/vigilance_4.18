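; Trigger-volume actor that shows an on-screen tip while the player character stands inside its box.
; On BeginPlay it creates a hidden TipsUI widget initialized with the actor's TipsText.
; Box overlap events, filtered to Player_CharacterBP, show the widget and add it to the viewport on entry, then hide and remove it on exit.
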(event OnComponentBeginOverlap(Box)
  (params (OverlappedComponent :type Primitive%20Component%20Object%20Reference) (OtherActor :type Actor%20Object%20Reference) (OtherComp :type Primitive%20Component%20Object%20Reference) (OtherBodyIndex :type Integer) (bFromSweep :type Boolean) (SweepResult :type Hit%20Result%20Structure%20%28by%20ref%29))
  (bind _ui (Variables|Default|GetUI))
  (Utilities|Casting|CastToPlayer_CharacterBP OtherActor)
  (Widget|SetVisibility _ui "Visible")
  (UserInterface|Viewport|AddtoViewport _ui 0))

(event OnComponentEndOverlap(Box)
  (params (OverlappedComponent :type Primitive%20Component%20Object%20Reference) (OtherActor :type Actor%20Object%20Reference) (OtherComp :type Primitive%20Component%20Object%20Reference) (OtherBodyIndex :type Integer))
  (bind _ui (Variables|Default|GetUI))
  (Utilities|Casting|CastToPlayer_CharacterBP OtherActor)
  (Widget|SetVisibility _ui "Hidden")
  (Widget|RemovefromParent _ui))

(event EventBeginPlay
  (bind _returnvalue (UserInterface|CreateWidget "/Game/Blueprints/CustomBlueprints/TipsActor/TipsUI.TipsUI_C" 0 (Variables|Default|GetTips%20Text)))
  (Variables|Default|SetUI _returnvalue)
  (Widget|SetVisibility (Variables|Default|GetUI) "Hidden"))

(event Collision|EventActorBeginOverlap
  (params (OtherActor :type Actor%20Object%20Reference)))

(event EventTick
  (params (DeltaSeconds :type Float%20%28single-precision%29)))

(fn ConstructionScript)