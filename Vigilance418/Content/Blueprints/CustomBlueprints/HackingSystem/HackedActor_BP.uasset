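; Child-actor Blueprint that makes its parent pawn hackable, letting the player take control of it.
; It shows a HackUI widget while the parent is recently rendered and has health above zero, and forwards hack start/stop to it.
; When the UI reports completion, the player controller blends the view to the pawn and possesses it.
; An optional timeout, or LoosControl, returns view and possession to Player_CharacterBP after ControlTime.
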(event OnComponentBeginOverlap(Sphere)
  (params (OverlappedComponent :type Primitive%20Component%20Object%20Reference) (OtherActor :type Actor%20Object%20Reference) (OtherComp :type Primitive%20Component%20Object%20Reference) (OtherBodyIndex :type Integer) (bFromSweep :type Boolean) (SweepResult :type Hit%20Result%20Structure%20%28by%20ref%29)))

(event OnComponentEndOverlap(Sphere)
  (params (OverlappedComponent :type Primitive%20Component%20Object%20Reference) (OtherActor :type Actor%20Object%20Reference) (OtherComp :type Primitive%20Component%20Object%20Reference) (OtherBodyIndex :type Integer)))

(event Custom|Hacked
  (bind _returnvalue (Game|GetPlayerController 0))
  (bind _returnvalue_2 (Game|GetPlayerController 0))
  (Game|Player|SetViewTargetwithBlend _returnvalue_2 (Actor|GetParentActor) 0.2 "VTBlend_Cubic" 0.0 false)
  (Rendering|SetVisibility (Variables|Default|GetWidget) false false)
  (bind _aspawn (Utilities|Casting|CastToPawn (Actor|GetParentActor)))
  (Pawn|Possess _returnvalue_2 _aspawn)
  (Default|CallOnHacked)
  (if (Variables|Default|GetShould%20loos%20control%20on%20time%20out)
    (Utilities|FlowControl|Delay 0.2)
    (Default|StartHacking (Variables|Default|GetUI) false)
    (Utilities|FlowControl|Delay (Variables|Default|GetControl%20time))
    (Rendering|SetVisibility (Variables|Default|GetWidget) false false)
    (bind _outactors (Actor|GetAllActorsOfClass "/Game/Blueprints/PlayerBlueprint/Player_CharacterBP.Player_CharacterBP_C"))
    (Game|Player|SetViewTargetwithBlend _returnvalue (Utilities|Array|Get(acopy) _outactors) 0.2 "VTBlend_Cubic" 0.0 false)
    (Utilities|FlowControl|Delay 0.2)
    (Pawn|Possess _returnvalue (Utilities|Array|Get(acopy) _outactors))))

(event Custom|Loos%20Control
  (bind _returnvalue (Game|GetPlayerController 0))
  (Default|StartHacking (Variables|Default|GetUI) false)
  (Utilities|FlowControl|Delay (Variables|Default|GetControl%20time))
  (Rendering|SetVisibility (Variables|Default|GetWidget) false false)
  (bind _outactors (Actor|GetAllActorsOfClass "/Game/Blueprints/PlayerBlueprint/Player_CharacterBP.Player_CharacterBP_C"))
  (Game|Player|SetViewTargetwithBlend _returnvalue (Utilities|Array|Get(acopy) _outactors) 0.2 "VTBlend_Cubic" 0.0 false)
  (Utilities|FlowControl|Delay 0.2)
  (Pawn|Possess _returnvalue (Utilities|Array|Get(acopy) _outactors)))

(event Custom|Start%20Hacking
  (params (Is%20Hacking :type Boolean))
  (bind _ui (Variables|Default|GetUI))
  (if (> (Variables|/Game/Blueprints/HealthAndDamageComponent.HealthAndDamageComponent_C|GetHealth (Actor|GetComponentbyClass (Actor|GetParentActor) "/Game/Blueprints/HealthAndDamageComponent.HealthAndDamageComponent_C")) 0.0)
    (Utilities|IsValid _ui
      (:Is%20Valid
        (Default|StartHacking _ui Is%20Hacking)))
    (else
      (Utilities|IsValid _ui
        (:Is%20Valid
          (Default|StartHacking _ui false))))))

(event Custom|Show%20Hack%20Widget
  (params (Show%20? :type Boolean))
  (bind _widget (Variables|Default|GetWidget))
  (if (Class|Actor|WasRecentlyRendered (Actor|GetParentActor) 0.2)
    (if (> (Variables|/Game/Blueprints/HealthAndDamageComponent.HealthAndDamageComponent_C|GetHealth (Actor|GetComponentbyClass (Actor|GetParentActor) "/Game/Blueprints/HealthAndDamageComponent.HealthAndDamageComponent_C")) 0.0)
      (Rendering|SetVisibility _widget Show%20? false)
      (Variables|Default|SetCan%20be%20Hacked true)
      (else
        (Rendering|SetVisibility _widget false false :!label _label)
        (Variables|Default|SetCan%20be%20Hacked false)))
    (else
      (goto _label))))

(event EventBeginPlay
  (bind _returnvalue (UserInterface|CreateWidget "/Game/Blueprints/CustomBlueprints/HackingSystem/HackUI.HackUI_C"))
  (UserInterface|SetWidget (Variables|Default|GetWidget) _returnvalue)
  (bind _output_get (Variables|Default|SetUI _returnvalue))
  (EventDispatchers|BindEventtoDoneHacking _output_get (delegate Custom|Hacked)))

(event EventTick
  (params (DeltaSeconds :type Float%20%28single-precision%29)))

(fn ConstructionScript)