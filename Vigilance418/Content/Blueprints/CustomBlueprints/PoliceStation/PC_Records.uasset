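; Police station records computer that plays a one-time mission beat when a police bot enters its trigger box.
; It stops the bot, disables its input, blends the camera to itself and has its PC_ScreenRecords widget show the info.
; The widget's shown event, after a delay, restores input and bot view, reveals the Decks waypoint and updates the objective.
; It then calls LoosControl on the bot's hack child actor.
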(event OnComponentBeginOverlap(Box)
  (params (OverlappedComponent :type Primitive%20Component%20Object%20Reference) (OtherActor :type Actor%20Object%20Reference) (OtherComp :type Primitive%20Component%20Object%20Reference) (OtherBodyIndex :type Integer) (bFromSweep :type Boolean) (SweepResult :type Hit%20Result%20Structure%20%28by%20ref%29))
  (bind _asnew_shooter_ai_police_bot (Utilities|Casting|CastToNewShooterAI_PoliceBot OtherActor))
  (Variables|Default|SetBot _asnew_shooter_ai_police_bot)
  (Utilities|FlowControl|DoOnce false
    (:Completed
      (Input|DisableInput _asnew_shooter_ai_police_bot (Game|GetPlayerController 0))
      (Components|Movement|StopMovementImmediately (Variables|/Script/Engine.Character|GetCharacterMovement _asnew_shooter_ai_police_bot))
      (Utilities|FlowControl|Delay 0.5)
      (Game|Player|SetViewTargetwithBlend (Game|GetPlayerController 0) self 1.0 "VTBlend_Linear" 0.0 false)
      (Utilities|FlowControl|Delay 2.0)
      (Default|ShowInfo (Variables|Default|GetUI)))))

(event Custom|On%20Info%20Shown
  (bind _returnvalue (Game|GetPlayerController 0))
  (bind _bot (Variables|Default|GetBot))
  (Utilities|FlowControl|Delay 1e+01)
  (Input|EnableInput _bot _returnvalue)
  (Game|Player|SetViewTargetwithBlend _returnvalue _bot 1.0 "VTBlend_Linear" 0.0 false)
  (bind _outactors (Actor|GetAllActorsOfClass "/Game/Blueprints/CustomBlueprints/CatchingDecks/WayPointToDecks.WayPointToDecks_C"))
  (Default|ShowWayPoint (Utilities|Array|Get(acopy) _outactors) true)
  (bind _asgame_play_gm (Utilities|Casting|CastToGamePlay_GM (Game|GetGameMode)))
  (Default|UpdateMissionObjective _asgame_play_gm "Get to Decks")
  (Utilities|FlowControl|Delay 2.0)
  (bind _ashacked_actor_bp (Utilities|Casting|CastToHackedActor_BP (Variables|/Script/Engine.ChildActorComponent|GetChildActor (Variables|/Game/Blueprints/AI_Blueprint/ShooterAI/NewShooterAI/NewShooterAI.NewShooterAI_C|GetHack (Variables|Default|GetBot)))))
  (Default|LoosControl _ashacked_actor_bp))

(event EventBeginPlay
  (bind _returnvalue (UserInterface|CreateWidget "/Game/Blueprints/CustomBlueprints/PoliceStation/PC_ScreenRecords.PC_ScreenRecords_C"))
  (bind _output_get (Variables|Default|SetUI _returnvalue))
  (UserInterface|SetWidget (Variables|Default|GetWidget) _output_get)
  (EventDispatchers|BindEventtoOnInfoShown _output_get (delegate Custom|On%20Info%20Shown)))

(event Collision|EventActorBeginOverlap
  (params (OtherActor :type Actor%20Object%20Reference)))

(event EventTick
  (params (DeltaSeconds :type Float%20%28single-precision%29)))

(fn ConstructionScript)