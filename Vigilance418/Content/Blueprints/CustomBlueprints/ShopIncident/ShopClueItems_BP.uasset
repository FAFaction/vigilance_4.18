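; Shop incident clue item that briefly shows a pointer widget when the player's scanner reaches it.
; An overlap of its box with BoundyScannerForplayer calls ShowPointer, which makes the widget visible, waits on a fixed delay, then hides it, ignoring its visibility argument.
; On BeginPlay it binds to the scanned event of its Scanned child actor, but that handler is empty.
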(event OnComponentBeginOverlap(Box)
  (params (OverlappedComponent :type Primitive%20Component%20Object%20Reference) (OtherActor :type Actor%20Object%20Reference) (OtherComp :type Primitive%20Component%20Object%20Reference) (OtherBodyIndex :type Integer) (bFromSweep :type Boolean) (SweepResult :type Hit%20Result%20Structure%20%28by%20ref%29))
  (Utilities|Casting|CastToBoundyScannerForplayer OtherActor)
  (CallFunction|ShowPointer true))

(event Custom|On%20Scanned)

(event Custom|Show%20Pointer
  (params (bNewVisibility :type Boolean))
  (Rendering|SetVisibility (Variables|Default|GetWidget) true false)
  (Utilities|FlowControl|Delay 1e+01)
  (Rendering|SetVisibility (Variables|Default|GetWidget) false false))

(event EventBeginPlay
  (bind _asscanned (Utilities|Casting|CastToScanned (Variables|/Script/Engine.ChildActorComponent|GetChildActor (Variables|Default|GetChildActor))))
  (EventDispatchers|BindEventtoOnScanned _asscanned (delegate Custom|On%20Scanned)))

(event Collision|EventActorBeginOverlap
  (params (OtherActor :type Actor%20Object%20Reference)))

(event EventTick
  (params (DeltaSeconds :type Float%20%28single-precision%29)))

(fn ConstructionScript)