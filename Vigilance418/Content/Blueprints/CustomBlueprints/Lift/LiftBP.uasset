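; Lift actor with sliding doors that travels between its base position and a stop point.
; A timeline slides both doors, and LiftUp closes them, eases the cabin over with MoveComponentTo, then briefly reopens them.
; Debug-style keys 4 and 5 toggle travel and doors through FlipFlops.
; A player entering the Box trigger sends the first LiftBP found in the level down, not necessarily this instance.
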(event OnComponentBeginOverlap(Box)
  (params (OverlappedComponent :type Primitive%20Component%20Object%20Reference) (OtherActor :type Actor%20Object%20Reference) (OtherComp :type Primitive%20Component%20Object%20Reference) (OtherBodyIndex :type Integer) (bFromSweep :type Boolean) (SweepResult :type Hit%20Result%20Structure%20%28by%20ref%29))
  (Utilities|Casting|CastToPlayer_CharacterBP OtherActor)
  (bind _outactors (Actor|GetAllActorsOfClass "LiftBP_C"))
  (CallFunction|LiftUp (Utilities|Array|Get(acopy) _outactors) false))

(event Custom|Open%20Lift
  (params (Open :type Boolean))
  ;[1 1 1] Comment
  (if Open
    (bind (_direction _x __x) (Timeline|Open%20Lift%20Door Play)
      (:Update
        (Transformation|SetRelativeLocation (Variables|Default|GetDoor%20l) (Math|Vector|MakeVector _x -201.0 -198.0) false false)
        (Transformation|SetRelativeLocation (Variables|Default|GetDoor%20R) (Math|Vector|MakeVector __x -201.0 -198.0) false false)))
    (else
      (Timeline|Open%20Lift%20Door Reverse))))

(event Custom|Lift%20Up
  (params (UP%20? :type Boolean))
  (bind _staticmesh (Variables|Default|GetStaticMesh))
  (CallFunction|OpenLift false)
  (Utilities|FlowControl|Delay 1.0)
  (Components|MoveComponentTo _staticmesh (select UP%20? (+ (Variables|Default|GetLift%20Stop%20Point) "0, 0,200.000000") "0, 0,200.000000") (.rotation (Transformation|GetRelativeTransform _staticmesh)) true true 5.0 false)
  (CallFunction|OpenLift true)
  (Utilities|FlowControl|Delay 1.0)
  (CallFunction|OpenLift false))

(event EventBeginPlay)

(event Collision|EventActorBeginOverlap
  (params (OtherActor :type Actor%20Object%20Reference)))

(event EventTick
  (params (DeltaSeconds :type Float%20%28single-precision%29)))

(event Input|KeyboardEvents|4
  (params (Key :type Key%20Structure))
  (:Pressed
    (Utilities|FlowControl|FlipFlop
      (:A
        (CallFunction|LiftUp true))
      (:B
        (CallFunction|LiftUp false)))))

(event Input|KeyboardEvents|5
  (params (Key :type Key%20Structure))
  (:Pressed
    (Utilities|FlowControl|FlipFlop
      (:A
        (CallFunction|OpenLift true))
      (:B
        (CallFunction|OpenLift false)))))

(fn ConstructionScript)