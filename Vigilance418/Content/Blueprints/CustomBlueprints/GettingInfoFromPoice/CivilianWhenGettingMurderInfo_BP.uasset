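; Civilian character for a murder-witness scene, who reports to a police officer and then walks off toward the apartment interrogation trigger.
; BeginPlay fills its widget with a down-arrow indicator.
; ReachedTheCop plays timed dialogue through GamePlay_GM, blends the view, re-possesses the player character, then starts AIMoveTo.
; An unconnected chain holds a cop warning and the follow-the-civilian notification, objective and camera reset, so those never run.
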(event Custom|Reached%20The%20Cop
  (bind _returnvalue (Game|GetPlayerController 0))
  (Utilities|AddNewDialogue "Clivilian" "Hello Officer")
  (Utilities|FlowControl|Delay 2.0)
  (Utilities|AddNewDialogue "Clivilian" "I saw some guy from Zeno")
  (Utilities|FlowControl|Delay 2.0)
  (Utilities|AddNewDialogue "Clivilian" "He cummited the murder")
  (Utilities|FlowControl|Delay 2.0)
  (Utilities|AddNewDialogue "Clivilian" "I saw him in")
  (Utilities|FlowControl|Delay 0.2)
  (Utilities|AddNewDialogue)
  (bind _outactors (Actor|GetAllActorsOfClass "/Game/Blueprints/PlayerBlueprint/Player_CharacterBP.Player_CharacterBP_C"))
  (Game|Player|SetViewTargetwithBlend _returnvalue 0 0.5 "VTBlend_Linear" 0.3 false)
  (Pawn|Possess _returnvalue (Utilities|Array|Get(acopy) _outactors))
  (Utilities|FlowControl|Delay 2.0)
  (bind _outactors_2 (Actor|GetAllActorsOfClass "/Game/Blueprints/CustomBlueprints/ApatmentInterrogation/TriggerApartmentInterrogation.TriggerApartmentInterrogation_C"))
  (AI|AIMoveTo self "0, 0, 0" (Utilities|Array|Get(acopy) _outactors_2) 5.0 false))

(event EventBeginPlay
  (bind _returnvalue (UserInterface|CreateWidget "/Game/UI/IndicatorUI.IndicatorUI_C" 0 "/Game/GameContent/UI/SCI_FI_Components_v1/Textures/Icons1/Icon_Down1_T.Icon_Down1_T"))
  (UserInterface|SetWidget (Variables|Default|GetWidget) _returnvalue))

(fn ConstructionScript)