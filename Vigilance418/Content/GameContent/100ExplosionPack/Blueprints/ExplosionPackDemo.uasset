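; Demo actor for the explosion pack that continuously previews one particle effect from a list around its own location.
; A fast looping timer started on BeginPlay spawns the selected emitter at a randomly jittered offset.
; Tick polls the 1 and 2 keys to step backward and forward through the list with wraparound.
; A UIHint widget created at start displays the current effect's object name.
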(event Custom|CustomEvent_0
  ;[0 0 0] Particles generator
  (Effects|SpawnEmitteratLocation (Utilities|Array|Get(acopy) (Variables|Default|GetParticleList) (Variables|Default|Getcurrent_index)) (+ (Transformation|GetActorLocation) (Math|Vector|MakeVector (Math|Random|RandomFloatinRange -2e+01 2e+01) (Math|Random|RandomFloatinRange -5e+01 5e+01) (Math|Random|RandomFloatinRange 1e+01 4e+01))) "0.000000,0.000000,0.000000"))

(event EventBeginPlay
  ;[0 0 0] Particles generator
  (Utilities|Time|SetTimerbyEvent (delegate Custom|CustomEvent_0) 0.15 true)
  ;[0 0 0] Output
  (bind _returnvalue (UserInterface|CreateWidget "/Game/GameContent/100ExplosionPack/Blueprints/UIHint.UIHint_C"))
  (UserInterface|Viewport|AddtoViewport _returnvalue 0)
  (Rendering|Components|TextRender|SetText (Variables|/Game/GameContent/100ExplosionPack/Blueprints/UIHint.UIHint_C|Getex_name _returnvalue) (Utilities|Text|ToText(String) (Utilities|GetObjectName (Utilities|Array|Get(acopy) (Variables|Default|GetParticleList) (Variables|Default|Getcurrent_index))))))

(event EventTick
  (params (DeltaSeconds :type Float%20%28single-precision%29))
  (bind _returnvalue (Game|GetPlayerController 0))
  (bind _particlelist (Variables|Default|GetParticleList))
  ;[0 0 0] Input 1 or 2
  (if (Game|Player|WasInputKeyJustPressed _returnvalue "Two")
    ;[0 0 0] Next, previous index
    (bind _result (Math|Integer|IncrementInt (Variables|Default|Getcurrent_index))
      (:%20%20
        (if (Utilities|Array|IsValidIndex _particlelist _result)
          _
          (else
            (Variables|Default|Setcurrent_index 0)))
        ;[0 0 0] Output
        (Rendering|Components|TextRender|SetText (Variables|/Game/GameContent/100ExplosionPack/Blueprints/UIHint.UIHint_C|Getex_name (stale EventBeginPlay _returnvalue)) (Utilities|Text|ToText(String) (Utilities|GetObjectName (Utilities|Array|Get(acopy) (Variables|Default|GetParticleList) (Variables|Default|Getcurrent_index)))) :!label _label)))
    (elif (Game|Player|WasInputKeyJustPressed _returnvalue "One")
      (bind _result_2 (Math|Integer|DecrementInt (Variables|Default|Getcurrent_index))
        (:%20%20
          (if (Utilities|Array|IsValidIndex _particlelist _result_2)
            (goto _label)
            (else
              (Variables|Default|Setcurrent_index (Utilities|Array|LastIndex _particlelist))
              (goto _label))))))))

(fn ConstructionScript)