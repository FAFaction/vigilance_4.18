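; Scannable-character helper actor that gives its parent Character a green highlight and a bio widget when scanned.
; On BeginPlay, after a short delay, it creates the ScanBio_UI widget and mirrors the parent's skeletal mesh with a highlight material, animated via master pose.
; Highlight toggles both visuals, starts the widget's scan once per activation, and relays its text-shown event through OnTextShown.
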(event Custom|On%20Bio%20Shown
  (Default|CallOnTextShown))

(event EventBeginPlay
  (bind _skeletalmesh (Variables|Default|GetSkeletalMesh))
  (Utilities|FlowControl|Delay 0.2)
  (bind _returnvalue (UserInterface|CreateWidget "/Game/AI_BountyMenu/AI/Blueprints/Highlight/ObjectScan/ScanBio_UI.ScanBio_UI_C" 0 (Variables|Default|GetName) (Variables|Default|GetBio) (Variables|Default|GetImage)))
  (UserInterface|SetWidget (Variables|Default|GetWidget) _returnvalue)
  (bind _ascharacter (Utilities|Casting|CastToCharacter (Actor|GetParentActor)))
  (Variables|Default|SetCharacter _ascharacter)
  (Class|SkinnedMeshComponent|SetSkeletalMesh _skeletalmesh (Variables|/Script/Engine.SkinnedMeshComponent|GetSkeletalMesh (Variables|/Script/Engine.Character|GetMesh (Variables|Default|GetCharacter))) true)
  (Rendering|Material|SetMaterial _skeletalmesh 0 "/Game/AI_BountyMenu/AI/Blueprints/Highlight/Material/M_Highlight_Green.M_Highlight_Green")
  (Transformation|AttachComponentToComponent (Variables|Default|GetSkeletalMesh) (Variables|/Script/Engine.Character|GetMesh (Variables|Default|GetCharacter)) "None" "SnapToTarget" "SnapToTarget" "SnapToTarget" true)
  (Class|SkinnedMeshComponent|SetMasterPoseComponent (Variables|Default|GetSkeletalMesh) (Variables|/Script/Engine.Character|GetMesh (Variables|Default|GetCharacter))))

(event EventTick
  (params (DeltaSeconds :type Float%20%28single-precision%29)))

(event EventHighlight
  (params (Active :type Boolean))
  (Variables|Default|SetScanning%20? Active)
  (Rendering|SetVisibility (Variables|Default|GetSkeletalMesh) Active false)
  (Rendering|SetVisibility (Variables|Default|GetWidget) Active false)
  (if Active
    (Utilities|FlowControl|DoOnce false :!label _label
      (:Completed
        (bind _asscan_bio_ui (Utilities|Casting|CastToScanBio_UI (UserInterface|GetUserWidgetObject (Variables|Default|GetWidget))))
        (Default|StartScanning _asscan_bio_ui (Variables|Default|GetScanning%20?))
        (EventDispatchers|BindEventtoOnTextShown _asscan_bio_ui (delegate Custom|On%20Bio%20Shown))))
    (else
      (goto _label Reset))))

(fn ConstructionScript)