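; HighlightedBounty_BP is an actor parented to a Character that shows a scanner-style highlight and bounty markers.
; On BeginPlay it copies the character's mesh via master pose, applies a dynamic outline material colored by bounty status, and fills the bounty info UI.
; Highlight toggles the outline and, for bounties, the pointer widget, focusing it once.
; Tick shows bounty info only while highlighted, recently rendered and near the camera's yaw.
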(event Custom|Set%20outline%20settings
  (params (Color :type Linear%20Color%20Structure :default "(R=1.000000,G=1.000000,B=1.000000,A=1.000000)") (Thickness :type Float%20%28single-precision%29) (Has%20Bounty :type Boolean)))

(event EventBeginPlay
  (bind _ascharacter (Utilities|Casting|CastToCharacter (Actor|GetParentActor)))
  (Class|SkinnedMeshComponent|SetSkeletalMesh (Variables|Default|GetSkeletalMesh) (Variables|/Script/Engine.SkinnedMeshComponent|GetSkeletalMesh (Variables|/Script/Engine.Character|GetMesh _ascharacter)) true)
  (Class|SkinnedMeshComponent|SetMasterPoseComponent (Variables|Default|GetSkeletalMesh) (Variables|/Script/Engine.Character|GetMesh _ascharacter))
  (Transformation|AttachComponentToComponent (Variables|Default|GetSkeletalMesh) (Variables|/Script/Engine.Character|GetMesh _ascharacter) "None" "KeepRelative" "KeepRelative" "KeepRelative" false)
  (CallFunction|Highlight false)
  (bind _returnvalue (Rendering|Material|CreateDynamicMaterialInstance "/Game/AI_BountyMenu/AI/Blueprints/Highlight/BountryScanner/Material/M_Highlight.M_Highlight" :!class /Script/Engine.KismetMaterialLibrary))
  (Variables|Default|SetMaterial _returnvalue)
  (bind _returnvalue_2 (UserInterface|CreateWidget "/Game/AI_BountyMenu/AI/Blueprints/Highlight/BountryScanner/Bounty_Pointer.Bounty_Pointer_C" 0 "(R=1.000000,G=1.000000,B=1.000000,A=1.000000)"))
  (bind _output_get (Variables|Default|SetUI _returnvalue_2))
  (UserInterface|SetWidget (Variables|Default|GetWidget) _output_get)
  (Rendering|Material|SetMaterial (Variables|Default|GetSkeletalMesh) 0 (Variables|Default|GetMaterial))
  (if (not (Variables|Highlight|GetHas%20Bounty))
    (Rendering|Material|SetVectorParameterValue (Variables|Default|GetMaterial) "Highlight Color" (Variables|Highlight|GetHighlight%20Color) :!class /Script/Engine.MaterialInstanceDynamic)
    (Rendering|Material|SetScalarParameterValue (Variables|Default|GetMaterial) "Line thickness" (Variables|Highlight|GetHightlight%20Thickness) :!class /Script/Engine.MaterialInstanceDynamic)
    (Class|WidgetComponent|SetTintColorandOpacity (Variables|Default|GetWidget) (Variables|Highlight|GetHighlight%20Color))
    (else
      (Rendering|Material|SetVectorParameterValue (Variables|Default|GetMaterial) "Highlight Color" "(R=0.000000,G=0.057446,B=1.000000,A=1.000000)" :!class /Script/Engine.MaterialInstanceDynamic)
      (Rendering|Material|SetScalarParameterValue (Variables|Default|GetMaterial) "Line thickness" 1.0 :!class /Script/Engine.MaterialInstanceDynamic)
      (Class|WidgetComponent|SetTintColorandOpacity (Variables|Default|GetWidget) "(R=0.000000,G=0.000000,B=1.000000,A=1.000000)")))
  (bind _asbounty_info_ui (Utilities|Casting|CastToBountyInfoUI (UserInterface|GetUserWidgetObject (Variables|Default|GetInfo%20UI))))
  (Default|UpdateUIInfo _asbounty_info_ui (Variables|Info|GetBounty%20Stats) (Variables|Info|GetBounty%20Reward) (Variables|Info|GetBounty%20Name) (Variables|Info|GetBounty%20Info)))

(event EventTick
  (params (DeltaSeconds :type Float%20%28single-precision%29))
  (bind _info_ui (Variables|Default|GetInfo%20UI))
  (if (Variables|Default|GetHIghlighted%20?)
    (if (Class|Actor|WasRecentlyRendered (Actor|GetParentActor) 0.2)
      (if (< (Math|Float|Absolute(Float) (.yaw (Math|Rotator|Delta(Rotator) (Math|Rotator|FindLookatRotation (Transformation|GetActorLocation (Game|Player|GetPlayerPawn 0)) (Transformation|GetActorLocation)) (Pawn|GetControlRotation (Game|GetPlayerController 0) :!class /Script/Engine.Controller)))) 4e+01)
        (if (Variables|Highlight|GetHas%20Bounty)
          (Rendering|SetVisibility _info_ui true false)
          (else
            (Rendering|SetVisibility _info_ui false false :!label _label)))
        (else
          (goto _label)))
      (else
        (goto _label)))
    (else
      (goto _label))))

(event EventHighlight
  (params (Active :type Boolean))
  (bind _ui (Variables|Default|GetUI))
  (Rendering|SetVisibility (Variables|Default|GetSkeletalMesh) Active false)
  (if (Variables|Highlight|GetHas%20Bounty)
    (Rendering|SetVisibility (Variables|Default|GetWidget) Active false)
    (Utilities|FlowControl|DoOnce false :!label _label
      (:Completed
        (Utilities|IsValid _ui
          (:Is%20Valid
            (Default|FocusActor _ui)))))
    (else
      (goto _label Reset))))

(fn ConstructionScript)