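; Bounty scanner Blueprint for the player that highlights HighlightedBounty_BP actors and remembers one that carries a bounty.
; ScanStart shows a visual sphere and grows it with the overlap sphere via a timeline, highlighting and recording actors it reaches.
; Actors without a bounty lose their highlight when overlap ends, while bounty holders keep it.
; The scanned list clears when the timeline finishes; ScanStop hides the visual and reverses the expansion.
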(event OnComponentBeginOverlap(Sphere)
  (params (OverlappedComponent :type Primitive%20Component%20Object%20Reference) (OtherActor :type Actor%20Object%20Reference) (OtherComp :type Primitive%20Component%20Object%20Reference) (OtherBodyIndex :type Integer) (bFromSweep :type Boolean) (SweepResult :type Hit%20Result%20Structure%20%28by%20ref%29))
  (bind _ashighlighted_bounty_bp (Utilities|Casting|CastToHighlightedBounty_BP OtherActor))
  (if (Variables|Default|GetScanning)
    (Utilities|FlowControl|Sequence
      (:then_0
        (if (Variables|/Game/AI_BountyMenu/AI/Blueprints/Highlight/HighlightedBounty_BP.HighlightedBounty_BP_C|GetHas%20Bounty _ashighlighted_bounty_bp)
          (Variables|Default|SetActor%20With%20Bounty _ashighlighted_bounty_bp)))
      (:then_1
        (Utilities|Array|Add (Variables|Default|GetScanned%20Actors) _ashighlighted_bounty_bp)
        (Default|Highlight _ashighlighted_bounty_bp true)))))

(event OnComponentEndOverlap(Sphere)
  (params (OverlappedComponent :type Primitive%20Component%20Object%20Reference) (OtherActor :type Actor%20Object%20Reference) (OtherComp :type Primitive%20Component%20Object%20Reference) (OtherBodyIndex :type Integer))
  (bind _ashighlighted_bounty_bp (Utilities|Casting|CastToHighlightedBounty_BP OtherActor))
  (if (not (Variables|/Game/AI_BountyMenu/AI/Blueprints/Highlight/HighlightedBounty_BP.HighlightedBounty_BP_C|GetHas%20Bounty _ashighlighted_bounty_bp))
    (Default|Highlight _ashighlighted_bounty_bp false)))

(event Custom|Scan%20Start
  (bind _sphere (Variables|Default|GetSphere))
  (Variables|Default|SetScanning true)
  (Rendering|SetVisibility (Variables|Default|GetSphere1) true false)
  (bind _radius (Timeline|Expan%20Scan%20Radius PlayFromStart)
    (:Update
      (Transformation|SetRelativeScale3D _sphere (Math|Conversions|ToVector(Float) _radius))
      (Components|Sphere|SetSphereRadius _sphere 32.0 true)
      (Transformation|SetRelativeScale3D (Variables|Default|GetSphere1) (Math|Conversions|ToVector(Float) _radius)))
    (:Finished
      (Utilities|Array|Clear (Variables|Default|GetScanned%20Actors))
      (Rendering|SetVisibility (Variables|Default|GetSphere1) false false))))

(event Custom|Scan%20Stop
  (bind _sphere (Variables|Default|GetSphere))
  (Variables|Default|SetScanning false)
  (Rendering|SetVisibility (Variables|Default|GetSphere1) false false)
  (bind _radius (Timeline|Expan%20Scan%20Radius Reverse)
    (:Update
      (Transformation|SetRelativeScale3D _sphere (Math|Conversions|ToVector(Float) _radius))
      (Components|Sphere|SetSphereRadius _sphere 32.0 true)
      (Transformation|SetRelativeScale3D (Variables|Default|GetSphere1) (Math|Conversions|ToVector(Float) _radius)))
    (:Finished
      (Utilities|Array|Clear (Variables|Default|GetScanned%20Actors))
      (Rendering|SetVisibility (Variables|Default|GetSphere1) false false))))

(event EventBeginPlay)

(fn ConstructionScript)