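; Actor that manages the player's bounty mission list and the bounty menu UI.
; On BeginPlay it creates the BountyMenu_WB widget with a reference to itself and enables input, so M toggles the menu, mouse cursor and input mode.
; Add and remove events maintain the Bounty array, with a name-based duplicate check that effectively compares only the last entry.
; UpdateBountyInfo is an empty stub.
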(event Custom|Update%20Bounty%20Info)

(event EventBeginPlay
  (bind _returnvalue (UserInterface|CreateWidget "/Game/AI_BountyMenu/BountyMenu/BountyMenu_WB.BountyMenu_WB_C" 0 self))
  (bind _output_get (Variables|Default|SetBounty%20Menu%20WB _returnvalue))
  (UserInterface|Viewport|AddtoPlayerScreen _output_get)
  (Input|EnableInput (Game|GetPlayerController 0)))

(event EventRemoveBountyMission
  (params (Bounty%20Mission :type S%20Bounty%20Info%20Structure))
  (Utilities|Array|RemoveItem (Variables|Default|GetBounty) Bounty%20Mission))

(event EventAddBountyMission
  (params (Bounty%20Mission :type S%20Bounty%20Info%20Structure))
  (bind _mission_exist (CallFunction|CheckifMissionExist Bounty%20Mission))
  (if (not _mission_exist)
    (Utilities|Array|Add (Variables|Default|GetBounty) Bounty%20Mission)))

(event Input|KeyboardEvents|M
  (params (Key :type Key%20Structure))
  (bind _returnvalue (Game|GetPlayerController 0))
  (bind _bounty_menu_wb (Variables|Default|GetBounty%20Menu%20WB))
  (:Pressed
    (if (not (Variables|/Game/AI_BountyMenu/BountyMenu/BountyMenu_WB.BountyMenu_WB_C|GetUI%20Open _bounty_menu_wb))
      (Default|OpenorCloseUI _bounty_menu_wb true)
      (Variables|/Script/Engine.PlayerController|SetbShowMouseCursor _returnvalue true)
      (Input|SetInputModeGameandUI _returnvalue (Variables|Default|GetBounty%20Menu%20WB) "DoNotLock" false)
      (else
        (Default|OpenorCloseUI _bounty_menu_wb false)
        (Variables|/Script/Engine.PlayerController|SetbShowMouseCursor _returnvalue false)
        (Input|SetInputModeGameOnly _returnvalue)))))

(fn ConstructionScript)

(fn CheckifMissionExist
  (params (Bounty%20Mission :type S%20Bounty%20Info%20Structure))
  (for _array_element (Variables|Default|GetBounty)
    (if (Utilities|Enum|Equal(Enum) (.MissionName (Utilities|Struct|BreakS_BountyInfo _array_element)) (.MissionName (Utilities|Struct|BreakS_BountyInfo Bounty%20Mission)))
      (LocalVariables|SetHas%20Mission true)
      (else
        (LocalVariables|SetHas%20Mission false))))
  (if (LocalVariables|GetHas%20Mission)
    (return true)
    (else
      (return false))))